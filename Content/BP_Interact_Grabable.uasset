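; Interaction Blueprint that lets the player pick up, carry, rotate and inspect physics objects.
; Grab toggles between releasing and line-tracing from the camera to grab the hit component with a supplied PhysicsHandle.
; While holding, Tick keeps the handle target ahead of the camera, and turn and look inputs rotate the component.
; ToggleRotate disables physics on press and release without restoring it; rotation-restore and face-player nodes are unconnected.
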(event `self.ReceiveBeginPlay`
  (set `self.PlayerCamera` (`GameplayStatics.GetPlayerCameraManager` 0)))

(event `Grab`
  (params (PhysicsHandle :type "PhysicsHandleComponent Object Reference"))
  (bind _transformcomponent (`PlayerCameraManager.TransformComponent` (`self.PlayerCamera`)))
  (bind _returnvalue (`SceneComponent.K2_GetComponentLocation` _transformcomponent))
  (bind _output_get (set `self.HoldingTarget` PhysicsHandle))
  (if (`self.IsHolding`)
    (`PhysicsHandleComponent.ReleaseComponent` _output_get)
    (set `self.GrabDistance` 80.0)
    (set `self.IsHolding` false)
    (else
      (`KismetSystemLibrary.PrintString` "Hello")
      (bind (_outhit _returnvalue_2) (`KismetSystemLibrary.LineTraceSingle` :`Start` _returnvalue :`End` (+ _returnvalue (* (`KismetMathLibrary.GetForwardVector` (`SceneComponent.K2_GetComponentRotation` _transformcomponent)) 200.0)) :`TraceChannel` "TraceTypeQuery1" :`DrawDebugType` "ForOneFrame"))
      (if _returnvalue_2
        (bind (_bblockinghit _binitialoverlap _time _distance _location _impactpoint _normal _impactnormal _physmat _hitactor _hitcomponent) (`GameplayStatics.BreakHitResult` _outhit))
        (`PhysicsHandleComponent.GrabComponentAtLocationWithRotation` :`self` (`self.HoldingTarget`) :`Component` _hitcomponent :`Location` _location)
        (set `self.IsHolding` true)
        (`KismetSystemLibrary.PrintString` "ICHGRefife")))))

(event `EnhancedInput|/Game/FPPuzzleGame/Input/IA_Turn`
  (params (ActionValue :type "Float (double-precision)") (ElapsedSeconds :type "Float (double-precision)") (TriggeredSeconds :type "Float (double-precision)") (InputAction :type "InputAction Object Reference" :default "/Game/FPPuzzleGame/Input/IA_Turn.IA_Turn"))
  (:`Triggered`
    (if (`self.IsHolding`)
      (`SceneComponent.K2_AddRelativeRotation` (`.HitComponent` (`GameplayStatics.BreakHitResult` (stale `Grab` _outhit))) (`KismetMathLibrary.MakeRotator` ActionValue) false false))))

(event `self.ReceiveTick`
  (params (DeltaSeconds :type "Float (single-precision)"))
  (bind _holdingtarget (`self.HoldingTarget`))
  (bind _transformcomponent (`PlayerCameraManager.TransformComponent` (`self.PlayerCamera`)))
  ;[0 1 0.7656] Turn to player
  (if (`self.IsHolding`)
    (`/Engine/EditorBlueprintResources/StandardMacros.IsValid` _holdingtarget
      (:`Is Valid`
        (`PhysicsHandleComponent.SetTargetLocation` _holdingtarget (+ (`SceneComponent.K2_GetComponentLocation` _transformcomponent) (* (`KismetMathLibrary.GetForwardVector` (`SceneComponent.K2_GetComponentRotation` _transformcomponent)) (`self.GrabDistance`))))
        (if true
          _
          (elif true
            _))))))

(event `EnhancedInput|/Game/FPPuzzleGame/Input/IA_LookUpDown`
  (params (ActionValue :type "Float (double-precision)") (ElapsedSeconds :type "Float (double-precision)") (TriggeredSeconds :type "Float (double-precision)") (InputAction :type "InputAction Object Reference" :default "/Game/FPPuzzleGame/Input/IA_LookUpDown.IA_LookUpDown"))
  (:`Triggered`
    (if (`self.IsHolding`)
      (`SceneComponent.K2_AddRelativeRotation` (`.HitComponent` (`GameplayStatics.BreakHitResult` (stale `Grab` _outhit))) (`KismetMathLibrary.MakeRotator` 0.0 ActionValue) false false))))

(event `EnhancedInput|/Game/FPPuzzleGame/Input/IA_ToggleRotate`
  (params (ActionValue :type Boolean) (ElapsedSeconds :type "Float (double-precision)") (TriggeredSeconds :type "Float (double-precision)") (InputAction :type "InputAction Object Reference" :default "/Game/FPPuzzleGame/Input/IA_ToggleRotate.IA_ToggleRotate"))
  (:`Started`
    (if (stale `Grab` _returnvalue_2)
      (if (`self.IsHolding`)
        (set `self.IsObjectInspecting` true)
        (bind (_bblockinghit _binitialoverlap _time _distance _location _impactpoint _normal _impactnormal _physmat _hitactor _hitcomponent) (`GameplayStatics.BreakHitResult` (stale `Grab` _outhit)))
        (`PrimitiveComponent.SetSimulatePhysics` _hitcomponent false))))
  (:`Completed`
    (if true
      (set `self.IsObjectInspecting` true)
      (`PrimitiveComponent.SetSimulatePhysics` _hitcomponent false)
      (set `self.RotationTarget` (`SceneComponent.K2_GetComponentRotation` _hitcomponent))
      (set `self.HasInspectedTarget` true))))