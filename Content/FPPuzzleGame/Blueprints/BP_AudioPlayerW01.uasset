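; BP_AudioPlayerW01 is a trigger actor in the puzzle game that plays an FMOD audio event the first time the player enters its box.
; BeginPlay assigns the NewEvent variable to the FMODAudio component.
; A Box overlap by any actor implementing BPI_Player passes through a DoOnce, which is never reset, to play that component.
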(event `self.ReceiveBeginPlay`
  (`FMODAudioComponent.SetEvent` (`self.FMODAudio`) (`self.New Event`)))

(event `self.Box.OnComponentBeginOverlap`
  (params (OverlappedComponent :type "PrimitiveComponent Object Reference") (OtherActor :type "Actor Object Reference") (OtherComp :type "PrimitiveComponent Object Reference") (OtherBodyIndex :type Integer) (bFromSweep :type Boolean) (SweepResult :type "HitResult Structure (by ref)"))
  (if (`KismetSystemLibrary.DoesImplementInterface` OtherActor "/Game/FPPuzzleGame/Blueprints/Interfaces/BPI_Player.BPI_Player_C")
    (`/Engine/EditorBlueprintResources/StandardMacros.DoOnce` false
      (:`Completed`
        (`FMODAudioComponent.Play` (`self.FMODAudio`))))))

(fn `UserConstructionScript`
  (set `self.New Event` (`self.New Event`)))