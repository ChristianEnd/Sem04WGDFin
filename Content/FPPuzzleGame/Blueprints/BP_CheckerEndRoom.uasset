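; BP_CheckerEndRoom is a puzzle checker, named for the end room, that tests whether linked actors' IsOn states match.
; Trigger runs CheckEqual, which requires Actor5 to match both Actor2 and Actor6, and Actor3 to match Actor4.
; On success, it sends a false bool message to each valid entry in TriggerActors and calls StopWhisper on GM_Gameplay inside that same loop.
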(event `/Game/FPPuzzleGame/Blueprints/Interfaces/BPI_Trigger.Trigger`
  (`self.CheckEqual`))

(event `CheckEqual`
  (if (== (`/Game/FPPuzzleGame/Blueprints/EnvironmentalAssets/BP_InteractTorchTorch.IsOn` (`self.Actor_5`)) (`/Game/FPPuzzleGame/Blueprints/EnvironmentalAssets/BP_InteractTorchTorch.IsOn` (`self.Actor_2`)))
    (if (== (`/Game/FPPuzzleGame/Blueprints/EnvironmentalAssets/BP_InteractTorchTorch.IsOn` (`self.Actor_3`)) (`/Game/FPPuzzleGame/Blueprints/EnvironmentalAssets/BP_InteractTorchTorch.IsOn` (`self.Actor_4`)))
      (if (== (`/Game/FPPuzzleGame/Blueprints/EnvironmentalAssets/BP_InteractTorchTorch.IsOn` (`self.Actor_5`)) (`/Game/FPPuzzleGame/Blueprints/EnvironmentalAssets/BP_InteractTorchTorch.IsOn` (`self.Actor_6`)))
        (for _array_element (`self.TriggerActors`)
          (`/Engine/EditorBlueprintResources/StandardMacros.IsValid` _array_element
            (:`Is Valid`
              (message `/Game/FPPuzzleGame/Blueprints/Interfaces/BPI_Trigger.TriggerWithBool` _array_element false)
              (bind _asgm_gameplay (cast `/Game/FPPuzzleGame/Blueprints/GameModes/GM_Gameplay` (`GameplayStatics.GetGameMode`)))
              (`/Game/FPPuzzleGame/Blueprints/GameModes/GM_Gameplay.StopWhisper` _asgm_gameplay))))))))

(fn `GetDisplayText`
  (returns (DisplayText :type String))
  (return ""))

(fn `UserConstructionScript`)