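; BP_PlacerRandomizer marks one random cube on each referenced BP_Placer with a red emissive wall material.
; Five seconds after BeginPlay it loops over PlacerReference, picks a random entry from each placer's ListOfCubes and swaps its static mesh material.
; The loop stops at the first entry that fails the cast to BP_Placer.
; An unconnected pair of debug line traces along ±Y from Cube never runs.
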(event `self.ReceiveBeginPlay`
  (`KismetSystemLibrary.Delay` 5.0)
  (for _array_element (`self.PlacerReference`)
    (bind _asbp_placer (cast `/Game/FPPuzzleGame/Blueprints/SchiebePuzzle/BP_Placer` _array_element))
    (bind _output_get (set `self.As BP Placer` _asbp_placer))
    (`/Engine/EditorBlueprintResources/StandardMacros.IsValid` _asbp_placer
      (:`Is Valid`
        (`PrimitiveComponent.SetMaterial` (`self.GetComponentByClass` (`KismetArrayLibrary.Array_Random` (`/Game/FPPuzzleGame/Blueprints/SchiebePuzzle/BP_Placer.ListOfCubes` _output_get)) "/Script/Engine.StaticMeshComponent") 0 "/Game/FPPuzzleGame/Materials/General/M_EmissiveWallsRed.M_EmissiveWallsRed")))))

(event `self.ReceiveTick`
  (params (DeltaSeconds :type "Float (single-precision)")))

(fn `UserConstructionScript`)