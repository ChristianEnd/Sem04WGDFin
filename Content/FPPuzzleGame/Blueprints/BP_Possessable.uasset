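; BP_Possessable is an interactable pawn the player can possess, using the minigame input mapping context.
; Interacting, while allowed, makes player controller 0 possess it and clears focus.
; Possession adds the mapping context and pushes a widget to the HUD's gameplay stack; unpossession removes the context and cleans the stack.
; Cancel input or a manual back call returns control to BP_Player.
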(event `SetInteractionDisabled`
  (set `self.CanBeInteractedWith` false))

(event `SetupInput`
  (params (PlayerController :type "PlayerController Object Reference"))
  ;[0.5 1 0] SetupInput
  (`EnhancedInputSubsystemInterface.AddMappingContext` (pcsubsystem `EnhancedInputLocalPlayerSubsystem` PlayerController) "/Game/FPPuzzleGame/Input/IMC_Minigame01.IMC_Minigame01" 0 (struct)))

(event `self.ReceivePossessed`
  (params (NewController :type "Controller Object Reference"))
  ;[0.4297 0 1] Possess
  (bind _asplayer_controller (cast `PlayerController` NewController))
  (`self.SetupInput` _asplayer_controller)
  (bind _pushedwidget (message `/Game/FPPuzzleGame/Blueprints/Interfaces/BPI_HUD.PushToGameplayStack` (`PlayerController.GetHUD` _asplayer_controller) (`self.Widget`)))
  (set `self.Pushed Widget` _pushedwidget))

(event `/Game/FPPuzzleGame/Blueprints/Interfaces/BPI_Interact.Interact`
  ;[0 0.2266 1] Interact
  (if (`self.CanBeInteractedWith`)
    (`Controller.Possess` (`GameplayStatics.GetPlayerController` 0) self)
    (`/Game/FPPuzzleGame/Blueprints/Interfaces/BPI_Interact.SetFocus` false)))

(event `self.ReceiveUnpossessed`
  (params (OldController :type "Controller Object Reference"))
  ;[0 0.5312 1] Unpossess
  (bind _asplayer_controller (cast `PlayerController` OldController :!label _label))
  (`EnhancedInputSubsystemInterface.RemoveMappingContext` (pcsubsystem `EnhancedInputLocalPlayerSubsystem` _asplayer_controller) "/Game/FPPuzzleGame/Input/IMC_Minigame01.IMC_Minigame01" (struct))
  (bind _returnvalue (`PlayerController.GetHUD` _asplayer_controller))
  (`/Engine/EditorBlueprintResources/StandardMacros.IsValid` _returnvalue
    (:`Is Valid`
      (message `/Game/FPPuzzleGame/Blueprints/Interfaces/BPI_HUD.CleanGameplayStack` _returnvalue "/Game/FPPuzzleGame/UI/Widgets/WBP_Gameplay.WBP_Gameplay_C"))))

(event `ManualUnposses`
  ;[0 0.5312 1] Unpossess
  (goto _label))

(event `EnhancedInput|/Game/FPPuzzleGame/Input/IA_Cancel`
  (params (ActionValue :type Boolean) (ElapsedSeconds :type "Float (double-precision)") (TriggeredSeconds :type "Float (double-precision)") (InputAction :type "InputAction Object Reference" :default "/Game/FPPuzzleGame/Input/IA_Cancel.IA_Cancel"))
  (bind _returnvalue (`GameplayStatics.GetPlayerController` 0))
  (:`Started`
    ;[1 0.4453 0] Back/Cancel
    (bind _returnvalue_2 (`GameplayStatics.GetActorOfClass` "/Game/FPPuzzleGame/Blueprints/Player/BP_Player.BP_Player_C" :!label _label_2))
    (`/Engine/EditorBlueprintResources/StandardMacros.IsValid` _returnvalue_2
      (:`Is Valid`
        (`/Engine/EditorBlueprintResources/StandardMacros.IsValid` _returnvalue
          (:`Is Valid`
            (`Controller.Possess` _returnvalue _returnvalue_2)
            (message `/Game/FPPuzzleGame/Blueprints/Interfaces/BPI_HUD.CleanGameplayStack` (`PlayerController.GetHUD` _returnvalue) "/Game/FPPuzzleGame/UI/Widgets/WBP_Gameplay.WBP_Gameplay_C")))))))

(event `ManualBackCall`
  (goto _label_2))

(fn `GetDisplayText`
  (returns (DisplayText :type String))
  (return ""))

(fn `UserConstructionScript`)