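; Possessable child actor that displays a configurable text message on a terminal widget in the puzzle game.
; After the parent's BeginPlay and Interact logic, it casts the pushed widget to WBP_Terminal and sets its DisplayText.
; Cancel input loops over referenced actors, firing TriggerMessage through BPI_Trigger where implemented and calling ManualBackCall for each valid one.
; Focus changes toggle custom depth rendering on its cube mesh.
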(event `self.ReceiveBeginPlay`
  (`parent.ReceiveBeginPlay`)
  (bind _aswbp_terminal (cast `/Game/FPPuzzleGame/UI/Widgets/WBP_Terminal` (`self.Pushed Widget`) :!label _label))
  (set `/Game/FPPuzzleGame/UI/Widgets/WBP_Terminal.DisplayText` (`self.Display Text`) _aswbp_terminal))

(event `self.ReceivePossessed`
  (params (NewController :type "Controller Object Reference"))
  (`parent.ReceivePossessed` NewController))

(event `/Game/FPPuzzleGame/Blueprints/Interfaces/BPI_Interact.Interact`
  (`parent.Interact`)
  (goto _label))

(event `EnhancedInput|/Game/FPPuzzleGame/Input/IA_Cancel`
  (params (ActionValue :type Boolean) (ElapsedSeconds :type "Float (double-precision)") (TriggeredSeconds :type "Float (double-precision)") (InputAction :type "InputAction Object Reference" :default "/Game/FPPuzzleGame/Input/IA_Cancel.IA_Cancel"))
  (:`Started`
    (for _array_element (`self.Actor`)
      (`/Engine/EditorBlueprintResources/StandardMacros.IsValid` _array_element
        (:`Is Valid`
          (if (`KismetSystemLibrary.DoesImplementInterface` _array_element "/Game/FPPuzzleGame/Blueprints/Interfaces/BPI_Trigger.BPI_Trigger_C")
            (message `/Game/FPPuzzleGame/Blueprints/Interfaces/BPI_Trigger.Trigger` _array_element))
          (`self.ManualBackCall`))))))

(event `/Game/FPPuzzleGame/Blueprints/Interfaces/BPI_Interact.SetFocus`
  (params (IsFocused :type Boolean))
  (`PrimitiveComponent.SetRenderCustomDepth` (`self.Cube1`) IsFocused))

(fn `UserConstructionScript`
  (`parent.UserConstructionScript`))