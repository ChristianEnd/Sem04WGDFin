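; BP_Socket is an interactable puzzle socket that holds an inventory item and notifies a linked actor when filled or emptied.
; Interact either returns the held item to the inventory or opens the inventory to place a selection, swapping the mesh from its DataTable row.
; Changes message the actor through BPI_Callable, falling back to BPI_Trigger, with ReverseCallMessage also sent on removal.
; CanPickUp, switchable by TriggerwithBool, gates interaction and custom-depth focus highlighting, while the construction script applies the preset item.
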(event `self.ReceiveBeginPlay`
  (if (`self.SlotTakenOnStart`)
    (`self.SetVis` false)
    (else
      (`self.SetVis` true))))

(event `/Game/FPPuzzleGame/Blueprints/Interfaces/BPI_Interact.SetFocus`
  (params (IsFocused :type Boolean))
  (bind _itemmesh (`self.ItemMesh`))
  (if (`self.CanPickUp`)
    (`PrimitiveComponent.SetRenderCustomDepth` _itemmesh IsFocused)
    (`PrimitiveComponent.SetRenderCustomDepth` (`self.PlaceInteractionCollider`) IsFocused)
    (else
      (`PrimitiveComponent.SetRenderCustomDepth` _itemmesh false)
      (`PrimitiveComponent.SetRenderCustomDepth` (`self.PlaceInteractionCollider`) false))))

(event `SelectItem`
  ;[1 1 1] OpenInventory
  (bind (_asbp_inv_rolando _fromsockettoinv) (`/Game/FPPuzzleGame/Library/BP_FunctionLibrary.OpenInventory` true))
  (set `/Game/FPPuzzleGame/UI/Widgets/BP_InvRolando.FromSocket` _fromsockettoinv _asbp_inv_rolando)
  (add `/Game/FPPuzzleGame/UI/Widgets/BP_InvRolando.OnItemSelected` _asbp_inv_rolando (delegate `ItemSelected`))
  (set `/Game/FPPuzzleGame/UI/Widgets/BP_InvRolando.CanUseItem` true _asbp_inv_rolando))

(event `/Game/FPPuzzleGame/Blueprints/Interfaces/BPI_Interact.Interact`
  (if (`self.CanPickUp`)
    (if (`self.SlotTakenOnStart`)
      (`/Game/FPPuzzleGame/Library/BP_FunctionLibrary.AddItemToInventory` (`self.Item`) 1)
      (`self.RemoveItem`)
      (`self.SetVis` true)
      (else
        (`self.SelectItem`)))))

(event `ItemSelected`
  (params (Item :type "/Game/FPPuzzleGame/Data/STRUCT_InventoryItem Structure"))
  ;[1 1 1] OpenInventory
  (bind _output_get (set `self.Item` Item_Item_5_FBAF9FAD491499507E90F5803292C23B))
  (set `self.Value/Amount` Item_Amount_6_F376C3734781C8B0EC26DC8E74BEC2C0)
  (`self.SetItem` _output_get)
  (`/Game/FPPuzzleGame/Library/BP_FunctionLibrary.RemoveItemFromInventory` _output_get 1))

(event `SetItem`
  (params (RowHandle :type "DataTableRowHandle Structure"))
  (bind (_datatable _rowname) (break `DataTableRowHandle` RowHandle))
  ;[1 1 1] SetItem
  (bind _returnvalue (`|GetDataTableRow` _datatable _rowname)
    (:`then`
      (bind _output_get (set `self.Out Row` _returnvalue))
      (`StaticMeshComponent.SetStaticMesh` (`self.ItemMesh`) (`.Mesh_8_BEC674D2464D70567BF325AD56A0041B` (break `/Game/FPPuzzleGame/Data/STRUCT_Item` _output_get)))
      (bind _output_get_2 (set `self.SlotTakenOnStart` true))
      (`self.CallAndTrigger`)
      (`self.SetVis` (not _output_get_2)))))

(event `SetVis`
  (params (bNewVisibility :type Boolean))
  ;[1 1 1] SetVis
  (`SceneComponent.SetVisibility` (`self.PlaceInteractionCollider`) bNewVisibility false))

(event `RemoveItem`
  ;[1 1 1] RemoveItem
  (`StaticMeshComponent.SetStaticMesh` (`self.ItemMesh`) null)
  (set `self.SlotTakenOnStart` false)
  (message `/Game/FPPuzzleGame/Blueprints/Interfaces/BPI_Callable.ReverseCall` (`self.Actor`))
  (`self.CallAndTrigger`))

(event `CallAndTrigger`
  (bind _actor (`self.Actor`))
  ;[1 1 1] CallAndTrigger
  (if (`KismetSystemLibrary.DoesImplementInterface` _actor "/Game/FPPuzzleGame/Blueprints/Interfaces/BPI_Callable.BPI_Callable_C")
    (message `/Game/FPPuzzleGame/Blueprints/Interfaces/BPI_Callable.Call` _actor self)
    (elif (`KismetSystemLibrary.DoesImplementInterface` _actor "/Game/FPPuzzleGame/Blueprints/Interfaces/BPI_Trigger.BPI_Trigger_C")
      (message `/Game/FPPuzzleGame/Blueprints/Interfaces/BPI_Trigger.Trigger` _actor))))

(event `/Game/FPPuzzleGame/Blueprints/Interfaces/BPI_Trigger.TriggerWithBool`
  (params (OnOff :type Boolean))
  (`KismetSystemLibrary.PrintString` "Socket")
  (set `self.CanPickUp` OnOff))

(fn `GetDisplayText`
  (returns (DisplayText :type String))
  (if (`self.SlotTakenOnStart`)
    (return "pick up")
    (else
      (return "place"))))

(fn `UserConstructionScript`
  (`self.SetItem` (`self.Item`)))