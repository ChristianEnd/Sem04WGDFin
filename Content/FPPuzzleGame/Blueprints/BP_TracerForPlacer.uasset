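; BP_TracerForPlacer is a puzzle sensor that detects a target material along the Y axis and triggers linked actors.
; Until solved, Tick line-traces from its Cube and compares the hit component's second material slot to MaterialToCompare.
; The first match fires CallMessage once on each Callable, marking it solved unless Bothways is set.
; With Bothways, a second trace, using a negated end Y coordinate, sets solved on its own match.
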(event `CheckMaterial`
  (bind (_bblockinghit _binitialoverlap _time _distance _location _impactpoint _normal _impactnormal _physmat _hitactor _hitcomponent) (`GameplayStatics.BreakHitResult` (stale `self.ReceiveTick` _outhit)))
  (`/Engine/EditorBlueprintResources/StandardMacros.IsValid` _hitcomponent
    (:`Is Valid`
      (if (== (`PrimitiveComponent.GetMaterial` _hitcomponent 1) (`self.MaterialToCompare`))
        (`/Engine/EditorBlueprintResources/StandardMacros.DoOnce` false
          (:`Completed`
            (for _array_element (`self.Callable`)
              (message `/Game/FPPuzzleGame/Blueprints/Interfaces/BPI_Callable.Call` _array_element null)
              (if (not (`self.Bothways?`))
                (set `self.IsSolved` true)))))))))

(event `self.ReceiveBeginPlay`)

(event `self.ReceiveTick`
  (params (DeltaSeconds :type "Float (single-precision)"))
  (bind _cube (`self.Cube`))
  (bind _tracedistance (`self.TraceDistance`))
  (bind (_returnvalue_x _returnvalue_y _returnvalue_z) (`KismetMathLibrary.BreakVector` (`SceneComponent.K2_GetComponentLocation` _cube)))
  (bind _returnvalue (`SceneComponent.K2_GetComponentLocation` _cube))
  (bind _returnvalue_2 (+ _returnvalue_y (select `bool` (`self.YP/YN`) :`false` (* _tracedistance -1.0) :`true` _tracedistance)))
  ;[1 1 1] TraceIfNeeded
  (if (not (`self.IsSolved`))
    (bind _outhit (`KismetSystemLibrary.LineTraceSingle` _returnvalue (`KismetMathLibrary.MakeVector` _returnvalue_x _returnvalue_2 _returnvalue_z) "TraceTypeQuery1"))
    (`self.CheckMaterial`)
    (if (`self.Bothways?`)
      (bind _outhit_2 (`KismetSystemLibrary.LineTraceSingle` _returnvalue (`KismetMathLibrary.MakeVector` _returnvalue_x (* _returnvalue_2 -1.0) _returnvalue_z) "TraceTypeQuery1"))
      (bind (_bblockinghit _binitialoverlap _time _distance _location _impactpoint _normal _impactnormal _physmat _hitactor _hitcomponent) (`GameplayStatics.BreakHitResult` _outhit_2))
      (`/Engine/EditorBlueprintResources/StandardMacros.IsValid` _hitcomponent
        (:`Is Valid`
          (if (== (`PrimitiveComponent.GetMaterial` _hitcomponent 1) (`self.MaterialToCompare`))
            (`KismetSystemLibrary.PrintString` "ImWinningDad" true true (struct :`G` 0.66 :`B` 1.0 :`A` 1.0) 5.0)
            (set `self.IsSolved` true)))))))

(fn `UserConstructionScript`)