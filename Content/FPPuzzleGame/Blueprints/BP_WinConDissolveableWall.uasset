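; Puzzle win-condition wall that dissolves and destroys itself when PuzzleSolved, Trigger or TriggerwithBool fires.
; Construction prepares a dynamic dissolve material but shows a distance-field opacity material until triggered.
; On trigger the cube swaps materials and a rate-adjusted timeline drives the Dissolve parameter before destroying the actor.
; A Select event clears custom-depth highlighting and steps an index through controlled actors, while the win-counter logic is unconnected.
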(event `self.ReceiveBeginPlay`
  ;[1 1 1] PlayRate
  (`TimelineComponent.SetPlayRate` (`self.Ani`) (`self.PlayRateDissolve`)))

(event `DissolveMaterial`
  ;[1 1 1] DissolveEvent
  (bind (_direction _alpha) (`Timeline|Ani` :!via `PlayFromStart`)
    (:`Update`
      (`MaterialInstanceDynamic.SetScalarParameterValue` (`self.M_Dynamic_Dissolve`) "Dissolve" (`KismetMathLibrary.Lerp` 1.0 -1.0 _alpha)))
    (:`Finished`
      (`self.K2_DestroyActor`))))

(event `self.PuzzleSolved`
  (`PrimitiveComponent.SetMaterial` (`self.Cube`) 0 (`self.M_Dynamic_Dissolve`) :!label _label)
  (`self.DissolveMaterial`))

(event `/Game/FPPuzzleGame/Blueprints/Interfaces/BPI_Trigger.Trigger`
  (goto _label))

(event `/Game/FPPuzzleGame/Blueprints/Interfaces/BPI_Trigger.TriggerWithBool`
  (params (OnOff :type Boolean))
  (goto _label))

(event `Select`
  (params (Direction :type "Float (double-precision)"))
  (bind _selected (`self.Selected`))
  (`|ExecutionSequence`
    (:`then_0`
      (`PrimitiveComponent.SetRenderCustomDepth` (`|GetArrayItem` (`self.K2_GetComponentsByClass` (`|GetArrayItem` (`self.ToControl`) (`self.Selected`)) "/Script/Engine.PrimitiveComponent")) false))
    (:`then_1`
      (if (> Direction 0.0)
        (set `self.Selected` (+ _selected 1))
        (else
          (set `self.Selected` (- _selected 1)))))))

(fn `UserConstructionScript`
  (bind _returnvalue (`KismetMaterialLibrary.CreateDynamicMaterialInstance` "/Game/FPPuzzleGame/Materials/Translucent/M_Dissolve_Red.M_Dissolve_Red"))
  (set `self.M_Dynamic_Dissolve` _returnvalue)
  (`PrimitiveComponent.SetMaterial` (`self.Cube`) 0 "/Game/FPPuzzleGame/Materials/DistanceFieldTest/M_DistanceFieldOpacity.M_DistanceFieldOpacity"))