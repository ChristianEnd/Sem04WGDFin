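; Character component that lets the player focus on and interact with objects in the first-person puzzle game.
; Each tick it sphere-traces forward from the owner's camera for actors implementing BPI_Interact.
; It tracks the current target, sending focus on/off messages and firing found/lost notifications as that changes.
; Interact sends the interact message to the focused actor through the interface, then clears the stored Character reference.
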(event `self.ReceiveBeginPlay`
  ;[0 1 0.8359] GetPlayerRefs
  (bind _ascharacter (cast `Character` (`self.GetOwner`)))
  (bind _output_get (set `self.Character` _ascharacter))
  (set `self.PlayerCamera` (`Actor.GetComponentByClass` _output_get "/Script/Engine.CameraComponent")))

(event `self.ReceiveTick`
  (params (DeltaSeconds :type "Float (single-precision)"))
  (`self.CheckForInteractables`))

(event `CheckForInteractables`
  ;[0 1 0.9063] CastFunctionality
  (bind _playercamera (`self.PlayerCamera`)
    (:`then`
      (bind _returnvalue (`SceneComponent.K2_GetComponentLocation` _playercamera))
      (bind _outhit (`KismetSystemLibrary.SphereTraceSingle` _returnvalue (+ _returnvalue (* (`SceneComponent.GetForwardVector` _playercamera) (`self.TraceDistance`))) (`self.TraceRadius`) "TraceTypeQuery1"))
      (bind (_bblockinghit _binitialoverlap _time _distance _location _impactpoint _normal _impactnormal _physmat _hitactor) (`GameplayStatics.BreakHitResult` _outhit))
      (if (`KismetSystemLibrary.DoesImplementInterface` _hitactor "/Game/FPPuzzleGame/Blueprints/Interfaces/BPI_Interact.BPI_Interact_C")
        (bind _currentinteractable (`self.CurrentInteractable`)
          (:`then`
            ;[1 0 0.9375] DeselectOldInteractable
            (if (!= _currentinteractable _hitactor)
              (bind _currentinteractable_2 (`self.CurrentInteractable` :!label _label)
                (:`then`
                  (message `/Game/FPPuzzleGame/Blueprints/Interfaces/BPI_Interact.SetFocus` _currentinteractable_2 false)
                  (`self.LostInteractable`)
                  (set `self.CurrentInteractable` null))
                (:`else`))))
          (:`else`
            ;[0.6641 1 0] SetNewInteractable
            (bind _output_get (set `self.CurrentInteractable` _hitactor))
            (message `/Game/FPPuzzleGame/Blueprints/Interfaces/BPI_Interact.SetFocus` _output_get true)
            (`self.FoundInteractable` _output_get)))
        (else
          (goto _label))))
    (:`else`)))

(event `Interact`
  ;[0.9453 1 0] Interact
  (bind _currentinteractable (`self.CurrentInteractable`)
    (:`then`
      (message `/Game/FPPuzzleGame/Blueprints/Interfaces/BPI_Interact.Interact` _currentinteractable)
      (set `self.Character` null))
    (:`else`)))