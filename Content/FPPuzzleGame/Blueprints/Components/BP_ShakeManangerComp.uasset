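; Actor component for first-person camera shakes, meant to switch between walk and idle shakes from the owning character's horizontal velocity.
; Each Tick checks that speed and calls ShakeCamera, which stops the old shake on a change and starts ActiveShake before updating it, even when unchanged.
; The cast that sets ActivePlayer is disconnected and BeginPlay is empty, so the validity check has no player assigned here.
; Older start/stop shake chains remain unconnected.
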(event `self.ReceiveBeginPlay`
  ;[0 0.8594 1] Init
)

(event `self.ReceiveTick`
  (params (DeltaSeconds :type "Float (single-precision)"))
  (`self.CheckPlayerWalkIdle`))

(event `CheckPlayerWalkIdle`
  ;[0.9311 1 0.1844] FPPlayerCameraShakes
  ;;[0.8516 1 0] WalkIdleState
  (bind _activeplayer (`self.ActivePlayer`)
    (:`then`
      (if (> (`KismetMathLibrary.VSizeXY` (`MovementComponent.Velocity` (`Character.CharacterMovement` _activeplayer))) 0.1)
        (`self.ShakeCamera` "/Game/FPPuzzleGame/Blueprints/Shakes/BP_WalkShake.BP_WalkShake_C")
        (set `self.ActiveShake` "/Game/FPPuzzleGame/Blueprints/Shakes/BP_WalkShake.BP_WalkShake_C")
        (else
          (`self.ShakeCamera` "/Game/FPPuzzleGame/Blueprints/Shakes/BP_IdleShake.BP_IdleShake_C")
          (set `self.ActiveShake` "/Game/FPPuzzleGame/Blueprints/Shakes/BP_IdleShake.BP_IdleShake_C"))))
    (:`else`)))

(event `ShakeCamera`
  (params (ShakeClass :type "CameraShakeBase Class Reference"))
  (bind _returnvalue (`GameplayStatics.GetPlayerCameraManager` 0))
  (if (!= ShakeClass (`self.ActiveShake`))
    (`PlayerCameraManager.StopCameraShake` _returnvalue (stale _returnvalue_2) true))
  (bind _returnvalue_2 (`PlayerCameraManager.StartCameraShakeFromSource` :`self` _returnvalue :`ShakeClass` (`self.ActiveShake`)))
  (set `self.ActiveShake` ShakeClass))