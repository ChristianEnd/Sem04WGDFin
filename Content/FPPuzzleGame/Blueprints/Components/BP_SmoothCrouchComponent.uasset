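; Character component meant to provide smooth crouching, though its crouch events currently drive nothing.
; BeginPlay caches the owning Character's capsule radius and standing and crouched half-heights.
; SmoothUncrouch checks headroom with a standing-sized capsule trace that draws debug shapes.
; Logic for lerping capsule height, toggling Crouch/UnCrouch by timeline direction and setting animation speed is present but never executed.
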(event `self.ReceiveBeginPlay`
  ;[0 0.625 1] GetCharacterInitInfos
  (bind _ascharacter (cast `Character` (`self.GetOwner`)))
  (set `self.CharacterRef` _ascharacter)
  (bind _capsulecomponent (`Character.CapsuleComponent` _ascharacter))
  (set `self.StandingHeight` (`CapsuleComponent.GetScaledCapsuleHalfHeight` _capsulecomponent))
  (set `self.Radius` (`CapsuleComponent.CapsuleRadius` _capsulecomponent))
  (set `self.CrouchedHeight` (`CharacterMovementComponent.CrouchedHalfHeight` (`Character.CharacterMovement` _ascharacter))))

(event `SmoothCrouch`
  ;[0.5234 0 1] CrouchUnCrouchFunc
)

(event `SmoothUncrouch`
  ;[0.5234 0 1] CrouchUnCrouchFunc
  (if (`self.CanUnCrouch`)
    _))

(fn `CanUnCrouch`
  (returns (CanUnCrouch :type Boolean))
  (bind _returnvalue (+ (`Actor.K2_GetActorLocation` (`self.CharacterRef`)) (`KismetMathLibrary.MakeVector` 0.0 0.0 (- (`self.StandingHeight`) (`self.CrouchedHeight`)))))
  (bind (_outhit _returnvalue_2) (`KismetSystemLibrary.CapsuleTraceSingle` :`Start` _returnvalue :`End` _returnvalue :`Radius` (`self.Radius`) :`HalfHeight` (`self.StandingHeight`) :`TraceChannel` "TraceTypeQuery1" :`DrawDebugType` "ForDuration"))
  (return (not _returnvalue_2)))