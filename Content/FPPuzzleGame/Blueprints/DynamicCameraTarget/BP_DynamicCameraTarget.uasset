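; BP_DynamicCameraTarget is a triggerable camera focus that temporarily pulls the view away from the player in a puzzle game.
; Trigger locks the cached BP_Player's look and walk, blends the player controller's view to a configured target, then waits a hold time.
; If blend-back is enabled, it blends back to the player and restores both controls after the blend.
; TriggerwithBool runs that same return path directly.
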(event `self.ReceiveBeginPlay`
  (bind _asbp_player (cast `/Game/FPPuzzleGame/Blueprints/Player/BP_Player` (`GameplayStatics.GetPlayerPawn` 0)))
  (set `self.As BP Player` _asbp_player))

(event `/Game/FPPuzzleGame/Blueprints/Interfaces/BPI_Trigger.TriggerWithBool`
  (params (OnOff :type Boolean))
  (bind _as_bp_player (`self.As BP Player`))
  (bind _blend_time (`self.Blend Time`))
  (`PlayerController.SetViewTargetWithBlend` (`GameplayStatics.GetPlayerController` 0) (`self.As BP Player`) _blend_time "VTBlend_Linear" 0.0 false :!label _label)
  (`KismetSystemLibrary.Delay` _blend_time)
  (set `/Game/FPPuzzleGame/Blueprints/Player/BP_Player.CanLook` true _as_bp_player)
  (set `/Game/FPPuzzleGame/Blueprints/Player/BP_Player.CanWalk` true _as_bp_player))

(event `/Game/FPPuzzleGame/Blueprints/Interfaces/BPI_Trigger.Trigger`
  (bind _as_bp_player (`self.As BP Player`))
  (set `/Game/FPPuzzleGame/Blueprints/Player/BP_Player.CanLook` false _as_bp_player)
  (set `/Game/FPPuzzleGame/Blueprints/Player/BP_Player.CanWalk` false _as_bp_player)
  (`PlayerController.SetViewTargetWithBlend` (`GameplayStatics.GetPlayerController` 0) (`self.New View Target`) (`self.Blend Time`) "VTBlend_Linear" 0.0 false)
  (`KismetSystemLibrary.Delay` (`self.HowLongToHold`))
  (if (`self.BlendBackAfterTime`)
    (goto _label)))

(fn `UserConstructionScript`)