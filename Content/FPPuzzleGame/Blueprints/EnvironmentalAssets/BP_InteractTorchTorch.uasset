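; Interactive torch that toggles between lit and unlit through Interact or Trigger, starting from its IsOn state.
; Lighting spawns a Niagara fire and fades in the light by timeline, then starts FMOD audio; extinguishing destroys the fire, fades out, then stops audio.
; DoOnce gates reset when the opposite fade finishes or, for lighting, its own fade finishes.
; Focus toggles custom depth on the torch mesh for highlighting.
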(event `self.ReceiveBeginPlay`
  (`LightComponent.SetIntensity` (`self.BP_FireLightComponent`) 0.0)
  (`TimelineComponent.SetPlayRate` (`self.AnimLightOff`) 6.0)
  (if (`self.IsOn`)
    (`self.TurnOn`)
    (else
      (`self.TurnOff`))))

(event `self.Trigger`
  (`self.StartFlame`))

(event `TurnOn`
  (bind _returnvalue (`NiagaraFunctionLibrary.SpawnSystemAtLocation` "/Game/FPPuzzleGame/VFX/Fire/NS_Fire.NS_Fire" (`SceneComponent.K2_GetComponentLocation` (`self.BP_FireLightComponent`)) :!label _label))
  (`/Engine/EditorBlueprintResources/StandardMacros.DoOnce` false :!label _label_2
    (:`Completed`
      (`NiagaraComponent.SetVariableFloat` _returnvalue "Size" 0.25)
      (bind (_direction _alpha) (`Timeline|AnimLight` :!via `PlayFromStart`)
        (:`Update`
          (`LightComponent.SetIntensity` (`self.BP_FireLightComponent`) (`KismetMathLibrary.Lerp` 0.0 1000.0 _alpha))
          (set `self.IsOn` true))
        (:`Finished`
          (`self.ResetTimelines2`)
          (`FMODAudioComponent.Play` (`self.FMODAudio`)))))))

(event `ResetTimelines2`
  (goto _label_2 :!via `Reset`))

(event `StartFlame`
  (if (not (`self.IsOn`))
    (goto _label)
    (else
      (`/Engine/EditorBlueprintResources/StandardMacros.IsValid` (stale `TurnOn` _returnvalue) :!label _label_3
        (:`Is Valid`
          (`/Engine/EditorBlueprintResources/StandardMacros.DoOnce` false :!label _label_4
            (:`Completed`
              (`ActorComponent.K2_DestroyComponent` (stale `TurnOn` _returnvalue))
              (bind (_direction _alpha) (`Timeline|AnimLightOff` :!via `PlayFromStart`)
                (:`Update`
                  (`LightComponent.SetIntensity` (`self.BP_FireLightComponent`) (`KismetMathLibrary.Lerp` 1000.0 0.0 _alpha))
                  (set `self.IsOn` false))
                (:`Finished`
                  (`self.ResetTimelines`)
                  (`FMODAudioComponent.Stop` (`self.FMODAudio`)))))))))))

(event `TurnOff`
  (goto _label_3))

(event `/Game/FPPuzzleGame/Blueprints/Interfaces/BPI_Interact.Interact`
  (`self.StartFlame`))

(event `ResetTimelines`
  (goto _label_4 :!via `Reset`))

(event `/Game/FPPuzzleGame/Blueprints/Interfaces/BPI_Interact.SetFocus`
  (params (IsFocused :type Boolean))
  (`PrimitiveComponent.SetRenderCustomDepth` (`self.Torch_low`) IsFocused))

(fn `GetDisplayText`
  (returns (DisplayText :type String))
  (return ""))

(fn `UserConstructionScript`)