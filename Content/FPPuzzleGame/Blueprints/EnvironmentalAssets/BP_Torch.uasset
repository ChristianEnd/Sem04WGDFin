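; BP_Torch is a torch actor that lights on BeginPlay when EnabledOnStart is set, or later through its Trigger event.
; StartFlame spawns a scaled-down Niagara fire at FlameCenter and plays the AnimLight timeline to fade BPFireLightComponent's intensity from zero toward MaxLuminosityCD.
; An optional AlternativeLightColor flag recolors the light during that timeline update, and an unlit torch starts with zero intensity.
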(event `self.ReceiveBeginPlay`
  (if (`self.EnabledOnStart`)
    (`self.StartFlame`)
    (else
      (`LightComponent.SetIntensity` (`self.BP_FireLightComponent`) 0.0))))

(event `/Game/FPPuzzleGame/Blueprints/Interfaces/BPI_Trigger.Trigger`
  (`self.StartFlame`))

(event `StartFlame`
  (bind _returnvalue (`NiagaraFunctionLibrary.SpawnSystemAtLocation` "/Game/FPPuzzleGame/VFX/Fire/NS_FIre1.NS_FIre1" (`SceneComponent.K2_GetComponentLocation` (`self.FlameCenter`))))
  (`NiagaraComponent.SetVariableFloat` _returnvalue "Size" 0.25)
  (bind (_direction _alpha) (`Timeline|AnimLight` :!via `PlayFromStart`)
    (:`Update`
      (`LightComponent.SetIntensity` (`self.BP_FireLightComponent`) (`KismetMathLibrary.Lerp` 0.0 (`self.MaxLuminosity(CD)`) _alpha))
      (if (`self.AlternativeLightColor`)
        (`LightComponent.SetLightColor` (`self.BP_FireLightComponent`) (`self.New Light Color`) true)
        (`LightComponent.SetLightColor` (`self.BP_FireLightComponent`) (`self.New Light Color`) true)))))

(fn `UserConstructionScript`)