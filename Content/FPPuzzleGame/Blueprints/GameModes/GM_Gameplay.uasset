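; Gameplay game mode for the puzzle game that caps the frame rate at 60 and manages 2D FMOD ambient audio.
; AudioEventAmbiance switches drone tracks; the standard drone starts at BeginPlay with a timeline-driven Volume fade-in.
; Switching it off only stores the instance for FadeOut, which nothing here calls.
; One-shot events start whispers and child laughter, though both laughter events play the standard drone.
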(event `self.ReceiveBeginPlay`
  (bind _returnvalue (`GameUserSettings.GetGameUserSettings`))
  (`GameUserSettings.SetFrameRateLimit` _returnvalue 60.0)
  (`self.AudioEventAmbiance` 0 true))

(event `AudioEventAmbiance`
  (params (Track :type Integer) (OnOff :type Boolean))
  (switch `int` Track
    (:`0`
      ;[1 1 1] 0 = StandardDroneAmbiance
      (if OnOff
        (`self.FadeIn`)
        (bind _returnvalue (`FMODBlueprintStatics.PlayEvent2D` "/Game/FMOD/Events/Ambiance/DroneAmbiances/StandardDrone.StandardDrone"))
        (set `self.ActiveSoundInstance` _returnvalue)
        (else
          (`|ExecutionSequence`
            (:`then_0`
              (set `self.OutFadeSound` (`self.ActiveSoundInstance`)))))))
    (:`1`
      ;[1 1 1] 1 = LabyrinthDrone
      (if OnOff
        (bind _returnvalue_2 (`FMODBlueprintStatics.PlayEvent2D` "/Game/FMOD/Events/Ambiance/DroneAmbiances/DroneLabyrinth.DroneLabyrinth"))
        (else
          (`FMODBlueprintStatics.EventInstanceStop` _returnvalue_2))))))

(event `PlayChildLaughingOne`
  (`/Engine/EditorBlueprintResources/StandardMacros.DoOnce` false
    (:`Completed`
      (`FMODBlueprintStatics.PlayEvent2D` "/Game/FMOD/Events/Ambiance/DroneAmbiances/StandardDrone.StandardDrone"))))

(event `FadeOut`
  (bind _outfadesound (`self.OutFadeSound`))
  ;[1 0.8726 0.4623] FadeControl
  (bind (_direction _alpha) (`Timeline|FadeOutAudio` :!via `PlayFromStart`)
    (:`Update`
      (`FMODBlueprintStatics.EventInstanceSetParameter` _outfadesound "Volume" (`KismetMathLibrary.Lerp` 100.0 0.0 _alpha)))
    (:`Finished`
      (`KismetSystemLibrary.Delay` 0.2)
      (`FMODBlueprintStatics.EventInstanceStop` _outfadesound))))

(event `PlayChildLaughingTwo`
  (`/Engine/EditorBlueprintResources/StandardMacros.DoOnce` false
    (:`Completed`
      (`FMODBlueprintStatics.PlayEvent2D` "/Game/FMOD/Events/Ambiance/DroneAmbiances/StandardDrone.StandardDrone"))))

(event `FadeIn`
  ;[1 0.8726 0.4623] FadeControl
  (bind (_direction _alpha) (`Timeline|FadeInAudio` :!via `PlayFromStart`)
    (:`Update`
      (`FMODBlueprintStatics.EventInstanceSetParameter` (`self.ActiveSoundInstance`) "Volume" (`KismetMathLibrary.Lerp` 0.0 100.0 _alpha)))))

(event `PlayWhisper`
  (`/Engine/EditorBlueprintResources/StandardMacros.DoOnce` false
    (:`Completed`
      (bind _returnvalue (`FMODBlueprintStatics.PlayEvent2D` "/Game/FMOD/Events/Ambiance/3DEvents/Voices.Voices")))))

(event `StopWhisper`
  (`FMODBlueprintStatics.EventInstanceStop` (stale `PlayWhisper` _returnvalue)))

(fn `UserConstructionScript`)