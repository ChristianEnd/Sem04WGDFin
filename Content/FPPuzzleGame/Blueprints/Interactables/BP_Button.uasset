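; Pressable puzzle button that responds to focus and interaction once an overlap with its radius flags a BPI_Player actor.
; Focus toggles custom depth on the button mesh, and interacting plays a timeline that slides it along X.
; When the timeline finishes, it sets IsActive, plays an optional level sequence and notifies its Manager through BPI_Callable.
; Its Interactable array is checked for BPI_Interact, but nothing is called on those actors.
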(event `self.ActRadius.OnComponentBeginOverlap`
  (params (OverlappedComponent :type "PrimitiveComponent Object Reference") (OtherActor :type "Actor Object Reference") (OtherComp :type "PrimitiveComponent Object Reference") (OtherBodyIndex :type Integer) (bFromSweep :type Boolean) (SweepResult :type "HitResult Structure (by ref)"))
  (bind _output_get (set `self.IsOverlappingWithPlayer` (`KismetSystemLibrary.DoesImplementInterface` OtherActor "/Game/FPPuzzleGame/Blueprints/Interfaces/BPI_Player.BPI_Player_C")))
  (if _output_get
    _))

(event `/Game/FPPuzzleGame/Blueprints/Interfaces/BPI_Interact.SetFocus`
  (params (IsFocused :type Boolean))
  (if (`self.IsOverlappingWithPlayer`)
    (`PrimitiveComponent.SetRenderCustomDepth` (`self.Button`) IsFocused)))

(event `/Game/FPPuzzleGame/Blueprints/Interfaces/BPI_Interact.Interact`
  (if (`self.IsOverlappingWithPlayer`)
    (bind (_direction _alpha) (`Timeline|Alpha` :`NewTime` 2.0 :!via `PlayFromStart`)
      (:`Update`
        (`SceneComponent.K2_SetRelativeLocation` (`self.Button`) (`KismetMathLibrary.MakeVector` (`KismetMathLibrary.Lerp` -49.999992 20.0 _alpha)) false false))
      (:`Finished`
        (`|ExecutionSequence`
          (:`then_0`
            (set `self.IsActive` (select `ETimelineDirection` _direction :`Forward` true)))
          (:`then_1`
            (for _array_element (`self.Interactable`)
              (`/Engine/EditorBlueprintResources/StandardMacros.IsValid` _array_element
                (:`Is Valid`
                  (if (`KismetSystemLibrary.DoesImplementInterface` _array_element "/Game/FPPuzzleGame/Blueprints/Interfaces/BPI_Interact.BPI_Interact_C")
                    _)))))
          (:`then_2`
            (bind _levelsequence (`self.LevelSequence`)
              (:`then`
                (`MovieSceneSequencePlayer.Play` (`LevelSequenceActor.SequencePlayer` _levelsequence)))
              (:`else`)))
          (:`then_3`
            (bind _manager (`self.Manager`)
              (:`then`
                (if (`KismetSystemLibrary.DoesImplementInterface` _manager "/Game/FPPuzzleGame/Blueprints/Interfaces/BPI_Callable.BPI_Callable_C")
                  (message `/Game/FPPuzzleGame/Blueprints/Interfaces/BPI_Callable.Call` _manager self)))
              (:`else`))))))))

(fn `UserConstructionScript`)