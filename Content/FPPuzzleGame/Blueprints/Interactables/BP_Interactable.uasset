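; BP_Interactable is a puzzle-game interactable that highlights via custom depth on focus and supplies interaction text.
; Interact opens the BP_InvRolando inventory when an item is configured, otherwise it just plays an optional level sequence.
; Selecting an item runs an optional item check with messages and inventory removal.
; That selection path can play the sequence and notify listed actors through BPI_Callable.
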(event `/Game/FPPuzzleGame/Blueprints/Interfaces/BPI_Interact.Interact`
  ;[1 1 1] Interact
  (`/Engine/EditorBlueprintResources/StandardMacros.IsValid` (break `DataTableRowHandle` (`.Item_5_FBAF9FAD491499507E90F5803292C23B` (break `/Game/FPPuzzleGame/Data/STRUCT_InventoryItem` (`self.Item`))))
    (:`Is Valid`
      (`self.OpenInv`))
    (:`Is Not Valid`
      (`self.PlaySequence`))))

(event `OpenInv`
  ;[1 1 1] OpenInventory
  (bind _pushedwidget (message `/Game/FPPuzzleGame/Blueprints/Interfaces/BPI_HUD.PushToGameplayStack` (`PlayerController.GetHUD` (`GameplayStatics.GetPlayerController` 0)) "/Game/FPPuzzleGame/UI/Widgets/BP_InvRolando.BP_InvRolando_C"))
  (bind _asbp_inv_rolando (cast `/Game/FPPuzzleGame/UI/Widgets/BP_InvRolando` _pushedwidget))
  (add `/Game/FPPuzzleGame/UI/Widgets/BP_InvRolando.OnItemSelected` _asbp_inv_rolando (delegate `ItemSelected`))
  (set `/Game/FPPuzzleGame/UI/Widgets/BP_InvRolando.CanUseItem` true _asbp_inv_rolando))

(event `ItemSelected`
  (params (Item :type "/Game/FPPuzzleGame/Data/STRUCT_InventoryItem Structure"))
  (bind _returnvalue (`PlayerController.GetHUD` (`GameplayStatics.GetPlayerController` 0)))
  (if (`self.NeedsItem`)
    ;[1 1 1] CheckItemIfNeeded
    (if (not (== (`.RowName` (break `DataTableRowHandle` Item_Item_5_FBAF9FAD491499507E90F5803292C23B)) (`.RowName` (break `DataTableRowHandle` (`.Item_5_FBAF9FAD491499507E90F5803292C23B` (break `/Game/FPPuzzleGame/Data/STRUCT_InventoryItem` (`self.Item`)))))))
      (message `/Game/FPPuzzleGame/Blueprints/Interfaces/BPI_HUD.ShowMessage` _returnvalue (make `/Game/FPPuzzleGame/Data/STRUCT_Message` "" "Wron Item"))
      (`/Game/FPPuzzleGame/Library/BP_FunctionLibrary.RemoveItemFromInventory` Item_Item_5_FBAF9FAD491499507E90F5803292C23B 1)
      (message `/Game/FPPuzzleGame/Blueprints/Interfaces/BPI_HUD.ShowMessage` _returnvalue (make `/Game/FPPuzzleGame/Data/STRUCT_Message` "" "Item Used"))
      (`|ExecutionSequence` :!label _label
        (:`then_0`
          (`self.PlaySequence`))
        (:`then_1`
          (`self.CallActor`))))
    (else
      (goto _label))))

(event `/Game/FPPuzzleGame/Blueprints/Interfaces/BPI_Interact.SetFocus`
  (params (IsFocused :type Boolean))
  (`PrimitiveComponent.SetRenderCustomDepth` (`self.Cube`) IsFocused))

(event `CallActor`
  ;[1 1 1] CallActor
  (if (`self.ShouldCallActor`)
    (for _array_element (`self.ActorToCall`)
      (`/Engine/EditorBlueprintResources/StandardMacros.IsValid` _array_element
        (:`Is Valid`
          (if (`KismetSystemLibrary.DoesImplementInterface` _array_element "/Game/FPPuzzleGame/Blueprints/Interfaces/BPI_Callable.BPI_Callable_C")
            (message `/Game/FPPuzzleGame/Blueprints/Interfaces/BPI_Callable.Call` _array_element null)))))))

(event `PlaySequence`
  (bind _levelsequence (`self.LevelSequence`))
  ;[1 1 1] Sequence
  (if (`self.ShouldPlaySequence`)
    (`/Engine/EditorBlueprintResources/StandardMacros.IsValid` _levelsequence
      (:`Is Valid`
        (`MovieSceneSequencePlayer.Play` (`LevelSequenceActor.SequencePlayer` _levelsequence))))))

(fn `GetDisplayText`
  (returns (DisplayText :type String))
  (return (`self.interactionText`)))

(fn `UserConstructionScript`)