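; BP_InteractionManager judges puzzle completion and fires the results on a list of target actors.
; In tracer mode, Call counts wins up to a threshold, then sends PuzzleSolvedMessage to the targets.
; Otherwise it compares each socket's item with the expected one, triggers targets on a match and makes the interact component ignore the last socket.
; Success also triggers a blend actor and sequence; ReverseCall switches targets off.
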(event `/Game/FPPuzzleGame/Blueprints/Interfaces/BPI_Callable.ReverseCall`
  (for _array_element (`self.Actors`)
    (message `/Game/FPPuzzleGame/Blueprints/Interfaces/BPI_Trigger.TriggerWithBool` _array_element false)))

(event `/Game/FPPuzzleGame/Blueprints/Interfaces/BPI_Callable.Call`
  (params (Actor :type "Actor Object Reference"))
  (if (`self.IsCheckingTracer`)
    (bind _result (`/Engine/EditorBlueprintResources/StandardMacros.IncrementInt` (`self.TracerWinCount`))
      (:`  `
        (bind _output_get (set `self.TracerWinCount` _result))
        (if (>= _output_get (`self.TracerWinCondition`))
          (for _array_element (`self.Actors`)
            (message `/Game/FPPuzzleGame/Blueprints/Interfaces/BPI_Puzzle.PuzzleSolved` _array_element)
            (`self.AfterEvents`)))))
    (else
      (set `self.IsCombinationRight` true)
      ;[1 1 1] CheckIfSocketHasRightItem
      (for _array_element_2 (`self.Items`)
        (bind (_socket _item) (break `/Game/FPPuzzleGame/Data/STRUCT_Socket` _array_element_2))
        (bind _asbp_socket (cast `/Game/FPPuzzleGame/Blueprints/BP_Socket` _socket))
        (bind (_item_datatable _item_rowname) (break `DataTableRowHandle` (`/Game/FPPuzzleGame/Blueprints/BP_Socket.Item` _asbp_socket)))
        (if (!= _item_rowname (`.RowName` (break `DataTableRowHandle` _item)))
          (set `self.IsCombinationRight` false)
          (`KismetSystemLibrary.PrintString` (`KismetSystemLibrary.GetDisplayName` _asbp_socket))))
      (`KismetSystemLibrary.PrintString` (`KismetStringLibrary.Conv_BoolToString` (`self.IsCombinationRight`)))
      (if (`self.IsCombinationRight`)
        (`self.AfterEvents`)
        (for _array_element_3 (`self.Actors`)
          (`/Engine/EditorBlueprintResources/StandardMacros.IsValid` _array_element_3
            (:`Is Valid`
              (message `/Game/FPPuzzleGame/Blueprints/Interfaces/BPI_Trigger.TriggerWithBool` _array_element_3 true)
              (`/Engine/EditorBlueprintResources/StandardMacros.IsValid` _asbp_socket
                (:`Is Valid`
                  (message `/Game/FPPuzzleGame/Blueprints/Interfaces/BPI_Trigger.TriggerWithBool` _asbp_socket false))))))
        (`/Game/FPPuzzleGame/Blueprints/Components/BP_InteractComp.AddToIgnore` (`self.GetComponentByClass` (`GameplayStatics.GetPlayerPawn` 0) "/Game/FPPuzzleGame/Blueprints/Components/BP_InteractComp.BP_InteractComp_C") _asbp_socket)
        (else
          (set `self.IsCombinationRight` false))))))

(event `AfterEvents`
  (bind _blendactor (`self.BlendActor`))
  (bind _sequence (`self.Sequence`))
  (`/Engine/EditorBlueprintResources/StandardMacros.IsValid` _blendactor
    (:`Is Valid`
      (message `/Game/FPPuzzleGame/Blueprints/Interfaces/BPI_Trigger.Trigger` _blendactor))
    (:`Is Not Valid`
      _))
  (`/Engine/EditorBlueprintResources/StandardMacros.IsValid` _sequence
    (:`Is Valid`
      (`MovieSceneSequencePlayer.Play` (`LevelSequenceActor.SequencePlayer` _sequence)))))

(fn `UserConstructionScript`)