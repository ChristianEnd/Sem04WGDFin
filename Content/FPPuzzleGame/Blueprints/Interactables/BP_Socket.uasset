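; BP_Socket is an interactable socket that holds one inventory item, which the player can take out or place.
; Interacting with a filled socket returns the item to the inventory and clears the mesh, while an empty one opens the inventory for selection.
; SetItem reads the mesh from the item's data table row, also in the construction script, and SlotTakenOnStart tracks occupancy.
; Focus toggles custom depth rendering on both meshes.
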(event `/Game/FPPuzzleGame/Blueprints/Interfaces/BPI_Interact.SetFocus`
  (params (IsFocused :type Boolean))
  (`PrimitiveComponent.SetRenderCustomDepth` (`self.Cylinder`) IsFocused)
  (`PrimitiveComponent.SetRenderCustomDepth` (`self.ItemMesh`) IsFocused))

(event `SelectItem`
  ;[1 1 1] OpenInventory
  (bind _asbp_inv_rolando (`/Game/FPPuzzleGame/Library/BP_FunctionLibrary.OpenInventory`))
  (add `/Game/FPPuzzleGame/UI/Widgets/BP_InvRolando.OnItemSelected` _asbp_inv_rolando (delegate `ItemSelected`))
  (set `/Game/FPPuzzleGame/UI/Widgets/BP_InvRolando.CanUseItem` true _asbp_inv_rolando))

(event `/Game/FPPuzzleGame/Blueprints/Interfaces/BPI_Interact.Interact`
  (if (`self.SlotTakenOnStart`)
    (`/Game/FPPuzzleGame/Library/BP_FunctionLibrary.AddItemToInventory` (`self.Item`) 1)
    (`self.RemoveItem`)
    (else
      (`self.SelectItem`)
      (`KismetSystemLibrary.PrintString` "SelectItem"))))

(event `ItemSelected`
  (params (Item :type "/Game/FPPuzzleGame/Data/STRUCT_InventoryItem Structure"))
  ;[1 1 1] OpenInventory
  (bind _output_get (set `self.Item` Item_Item_5_FBAF9FAD491499507E90F5803292C23B))
  (set `self.Value/Amount` Item_Amount_6_F376C3734781C8B0EC26DC8E74BEC2C0)
  (`self.SetItem` _output_get)
  (`/Game/FPPuzzleGame/Library/BP_FunctionLibrary.RemoveItemFromInventory` _output_get 1))

(event `SetItem`
  (params (RowHandle :type "DataTableRowHandle Structure"))
  (bind (_datatable _rowname) (break `DataTableRowHandle` RowHandle))
  ;[1 1 1] SetItem
  (bind _returnvalue (`|GetDataTableRow` _datatable _rowname)
    (:`then`
      (bind _output_get (set `self.Out Row` _returnvalue))
      (`StaticMeshComponent.SetStaticMesh` (`self.ItemMesh`) (`.Mesh_8_BEC674D2464D70567BF325AD56A0041B` (break `/Game/FPPuzzleGame/Data/STRUCT_Item` _output_get)))
      (set `self.SlotTakenOnStart` true))))

(event `RemoveItem`
  (`StaticMeshComponent.SetStaticMesh` (`self.ItemMesh`) null)
  (set `self.SlotTakenOnStart` false))

(fn `UserConstructionScript`
  (`self.SetItem` (`self.Item`)))