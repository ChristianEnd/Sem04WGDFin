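; BP_Item is a collectible pickup in the puzzle game, defined by a data table row that sets its mesh in the construction script.
; Focus toggles custom depth on the mesh, and GetDisplayText supplies the "to collect" prompt.
; Interact adds the item and amount to BP_Player's inventory component, shows a HUD message naming the item if its row is found, then destroys the actor.
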(event `/Game/FPPuzzleGame/Blueprints/Interfaces/BPI_Interact.SetFocus`
  (params (IsFocused :type Boolean))
  (`PrimitiveComponent.SetRenderCustomDepth` (`self.Mesh`) IsFocused))

(event `/Game/FPPuzzleGame/Blueprints/Interfaces/BPI_Interact.Interact`
  (bind (_datatable _rowname) (break `DataTableRowHandle` (`self.Item`)))
  (`|ExecutionSequence`
    (:`then_0`
      ;[1 0.5836 0.9726] AddItem
      (bind _returnvalue (`GameplayStatics.GetActorOfClass` "/Game/FPPuzzleGame/Blueprints/Player/BP_Player.BP_Player_C"))
      (`/Game/FPPuzzleGame/Blueprints/Components/BP_InventoryComponent.AddItem` (`/Game/FPPuzzleGame/Blueprints/Player/BP_Player.BP_InventoryComponent` _returnvalue) (`self.Item`) (`self.Value/Amount`)))
    (:`then_1`
      ;[0.431 1 0.9606] GenerateMessage
      (bind _returnvalue_2 (`|GetDataTableRow` _datatable _rowname)
        (:`then`
          (message `/Game/FPPuzzleGame/Blueprints/Interfaces/BPI_HUD.ShowMessage` (`PlayerController.GetHUD` (`GameplayStatics.GetPlayerController` 0)) (make `/Game/FPPuzzleGame/Data/STRUCT_Message` "Item collected" (`|FormatText` "You have collected a {name}" (`.Name_2_72B15ADF46FD7B53382652A1266672CA` (break `/Game/FPPuzzleGame/Data/STRUCT_Item` _returnvalue_2)))))
          (`self.K2_DestroyActor`))))
    (:`then_2`
      (`self.K2_DestroyActor`))))

(fn `GetDisplayText`
  (returns (DisplayText :type String))
  (return "to collect"))

(fn `UserConstructionScript`
  (bind (_datatable _rowname) (break `DataTableRowHandle` (`self.Item`)))
  (bind _returnvalue (`|GetDataTableRow` _datatable _rowname)
    (:`then`
      (`StaticMeshComponent.SetStaticMesh` (`self.Mesh`) (`.Mesh_8_BEC674D2464D70567BF325AD56A0041B` (break `/Game/FPPuzzleGame/Data/STRUCT_Item` _returnvalue))))))