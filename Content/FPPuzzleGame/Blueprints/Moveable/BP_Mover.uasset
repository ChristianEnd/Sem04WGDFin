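; BP_Mover is a puzzle actor that, on interaction, moves a list of actors to paired target locations and plays an optional level sequence.
; A timeline with adjustable play rate lerps each actor from its current location, so motion compounds each update, then calls an empty AfterAnimation hook.
; It also shows a reference material on its cube and counts reported meshes with that material up to Condition, without acting on the count.
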(event `self.ReceiveBeginPlay`
  ;[1 1 1] SetPlayRate
  (`TimelineComponent.SetPlayRate` (`self.Anim`) (`self.PlayRate`))
  (`PrimitiveComponent.SetMaterial` (`self.Cube1`) 0 (`self.MaterialToCompare`)))

(event `/Game/FPPuzzleGame/Blueprints/Interfaces/BPI_Interact.SetFocus`
  (params (IsFocused :type Boolean)))

(event `AfterAnimation`)

(event `/Game/FPPuzzleGame/Blueprints/Interfaces/BPI_Interact.Interact`
  (bind _actorstomove (`self.ActorsToMove`))
  (bind _levelsequence (`self.LevelSequence`))
  (`|ExecutionSequence`
    (:`then_0`
      ;[1 1 1] ActorToMove
      (bind (_direction _alpha) (`Timeline|Anim` :!via `PlayFromStart`)
        (:`Update`
          (for (_array_element _array_index) _actorstomove
            (if (`KismetArrayLibrary.Array_IsValidIndex` _actorstomove _array_index)
              (`self.K2_SetActorLocation` _array_element (`KismetMathLibrary.VLerp` (`self.K2_GetActorLocation` _array_element) (`|GetArrayItem` (`self.Locations`) _array_index) _alpha) false false))))
        (:`Finished`
          (`self.AfterAnimation`))))
    (:`then_1`
      ;[1 1 1] PlayLevelSequence
      (`/Engine/EditorBlueprintResources/StandardMacros.IsValid` _levelsequence
        (:`Is Valid`
          (`MovieSceneSequencePlayer.Play` (`LevelSequenceActor.SequencePlayer` _levelsequence)))))))

(event `/Game/FPPuzzleGame/Blueprints/Interfaces/BPI_Puzzle.PuzzleAddWithActor`
  (params (StaticMesh :type "StaticMesh Object Reference"))
  ;[1 1 1] AfterBlock
  (if (== (`StaticMesh.GetMaterial` StaticMesh 0) (`self.MaterialToCompare`))
    (if (not (== (`self.Count`) (`self.Condition`)))
      (set `self.Count` (+ (`self.Count`) 1)))))

(fn `UserConstructionScript`)