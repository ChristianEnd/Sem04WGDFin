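; Interactable control pawn for the turnables puzzle minigame, which the player possesses on interact and leaves on cancel to return to BP_Player.
; Possession adds IMC_TurnablesMiniGame and switches the HUD to the terminal widget, while unpossession removes a different context, IMC_Minigame01, and restores the gameplay widget.
; Move, scroll and rotate-toggle inputs drive TargetToSolveMoveableCollider to shift, turn or flip, tracking a wrapping three-step position that resets on flip.
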(event `self.ReceiveUnpossessed`
  (params (OldController :type "Controller Object Reference"))
  ;[1 0 0.1875] Unpossess
  (bind _asplayer_controller (cast `PlayerController` OldController))
  (`EnhancedInputSubsystemInterface.RemoveMappingContext` (pcsubsystem `EnhancedInputLocalPlayerSubsystem` _asplayer_controller) "/Game/FPPuzzleGame/Input/IMC_Minigame01.IMC_Minigame01" (struct))
  (message `/Game/FPPuzzleGame/Blueprints/Interfaces/BPI_HUD.CleanGameplayStack` (`PlayerController.GetHUD` _asplayer_controller) "/Game/FPPuzzleGame/UI/Widgets/WBP_Gameplay.WBP_Gameplay_C"))

(event `self.ReceivePossessed`
  (params (NewController :type "Controller Object Reference"))
  ;[0 0.01562 1] Possess
  (bind _asplayer_controller (cast `PlayerController` NewController))
  (`self.SetupInput` _asplayer_controller)
  (message `/Game/FPPuzzleGame/Blueprints/Interfaces/BPI_HUD.PushToGameplayStack` (`PlayerController.GetHUD` _asplayer_controller) "/Game/FPPuzzleGame/UI/Widgets/WBP_Terminal.WBP_Terminal_C"))

(event `/Game/FPPuzzleGame/Blueprints/Interfaces/BPI_Interact.SetFocus`
  (params (IsFocused :type Boolean))
  (`PrimitiveComponent.SetRenderCustomDepth` (`self.Interactable`) IsFocused))

(event `/Game/FPPuzzleGame/Blueprints/Interfaces/BPI_Interact.Interact`
  ;[0.8047 0 1] Interact
  (`Controller.Possess` (`GameplayStatics.GetPlayerController` 0) self)
  (`PrimitiveComponent.SetRenderCustomDepth` (`self.Interactable`) false))

(event `SetupInput`
  (params (PlayerController :type "PlayerController Object Reference"))
  ;[0 0.7422 1] SetupInput
  (`EnhancedInputSubsystemInterface.AddMappingContext` (pcsubsystem `EnhancedInputLocalPlayerSubsystem` PlayerController) "/Game/FPPuzzleGame/Input/IMC_TurnablesMiniGame.IMC_TurnablesMiniGame" 0 (struct)))

(event `EnhancedInput|/Game/FPPuzzleGame/Input/IA_Cancel`
  (params (ActionValue :type Boolean) (ElapsedSeconds :type "Float (double-precision)") (TriggeredSeconds :type "Float (double-precision)") (InputAction :type "InputAction Object Reference" :default "/Game/FPPuzzleGame/Input/IA_Cancel.IA_Cancel"))
  (bind _returnvalue (`GameplayStatics.GetPlayerController` 0))
  ;[0 0.9297 1] BackOut
  (:`Started`
    (bind _returnvalue_2 (`GameplayStatics.GetActorOfClass` "/Game/FPPuzzleGame/Blueprints/Player/BP_Player.BP_Player_C"))
    (`Controller.Possess` _returnvalue _returnvalue_2)
    (message `/Game/FPPuzzleGame/Blueprints/Interfaces/BPI_HUD.CleanGameplayStack` (`PlayerController.GetHUD` _returnvalue) "/Game/FPPuzzleGame/UI/Widgets/WBP_Gameplay.WBP_Gameplay_C")))

(event `EnhancedInput|/Game/FPPuzzleGame/Input/IA_MoveLeftRight`
  (params (ActionValue :type "Float (double-precision)") (ElapsedSeconds :type "Float (double-precision)") (TriggeredSeconds :type "Float (double-precision)") (InputAction :type "InputAction Object Reference" :default "/Game/FPPuzzleGame/Input/IA_MoveLeftRight.IA_MoveLeftRight"))
  (bind _targettosolvemoveablecollider (`self.TargetToSolveMoveableCollider`))
  (bind _targettosolvemoveablecollider_2 (`self.TargetToSolveMoveableCollider`))
  ;[0 0.0625 1] MoveLeftRight
  (:`Started`
    (if (> ActionValue 0.0)
      (bind _output_get (set `self.Position Int` (+ (`self.Position Int`) 1)))
      (if (== _output_get 2)
        (bind _output_get_2 (set `self.Position Int` -1))
        (`/Game/FPPuzzleGame/Blueprints/Puzzle01Turnables/MoveableCollider/BP_MoveableCollider.MoveUp/Right` _targettosolvemoveablecollider _output_get_2)
        (else
          (`/Game/FPPuzzleGame/Blueprints/Puzzle01Turnables/MoveableCollider/BP_MoveableCollider.MoveUp/Right` _targettosolvemoveablecollider _output_get)))
      (else
        (bind _output_get_3 (set `self.Position Int` (- (`self.Position Int`) 1)))
        (if (== _output_get_3 -2)
          (bind _output_get_4 (set `self.Position Int` 1))
          (`/Game/FPPuzzleGame/Blueprints/Puzzle01Turnables/MoveableCollider/BP_MoveableCollider.MoveUp/Right` _targettosolvemoveablecollider_2 _output_get_4)
          (else
            (`/Game/FPPuzzleGame/Blueprints/Puzzle01Turnables/MoveableCollider/BP_MoveableCollider.MoveDown/Lef` _targettosolvemoveablecollider_2 _output_get_3)))))))

(event `EnhancedInput|/Game/FPPuzzleGame/Input/IA_Scroll`
  (params (ActionValue :type "Float (double-precision)") (ElapsedSeconds :type "Float (double-precision)") (TriggeredSeconds :type "Float (double-precision)") (InputAction :type "InputAction Object Reference" :default "/Game/FPPuzzleGame/Input/IA_Scroll.IA_Scroll"))
  ;[1 0.7969 0] ScrollTurn
  (:`Started`
    (`/Game/FPPuzzleGame/Blueprints/Puzzle01Turnables/MoveableCollider/BP_MoveableCollider.Turn` (`self.TargetToSolveMoveableCollider`) ActionValue)))

(event `EnhancedInput|/Game/FPPuzzleGame/Input/IA_ToggleRotate`
  (params (ActionValue :type Boolean) (ElapsedSeconds :type "Float (double-precision)") (TriggeredSeconds :type "Float (double-precision)") (InputAction :type "InputAction Object Reference" :default "/Game/FPPuzzleGame/Input/IA_ToggleRotate.IA_ToggleRotate"))
  (:`Started`
    (bind _output_get (set `self.IsHorizontal` ActionValue))
    (`/Game/FPPuzzleGame/Blueprints/Puzzle01Turnables/MoveableCollider/BP_MoveableCollider.FlipIt` (`self.TargetToSolveMoveableCollider`) _output_get)
    (set `self.Position Int` 0)))

(fn `NewFunction`)

(fn `UserConstructionScript`)