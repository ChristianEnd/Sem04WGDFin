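; Turnable cube puzzle actor in which the player picks one of three rows or columns and scrolls to rotate its pieces.
; Left/right input cycles the TraceHolder position, and interact flips it between horizontal and vertical.
; Each tick a left multi-line trace highlights hits via custom depth and stores their actors, which scroll turns 90 degrees on yaw or roll through one RInterpTo call.
; Middle and right traces are empty, their logic disconnected.
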(event `self.ReceiveTick`
  (params (DeltaSeconds :type "Float (single-precision)"))
  (set `self.Delta Seconds` DeltaSeconds)
  (`self.FocusSelected`))

(event `TraceMid`
  ;[1 1 1] Traces
)

(event `FocusSelected`
  (`self.TraceMid`)
  (`self.TraceLeft`)
  (`self.TraceRight`))

(event `TraceLeft`
  (bind _returnvalue (`SceneComponent.K2_GetComponentLocation` (`self.TraceStartLeft`)))
  ;[1 1 1] Traces
  (bind _outhits (`KismetSystemLibrary.LineTraceMulti` :`Start` _returnvalue :`End` (+ _returnvalue (0.0 -400.0 0.0)) :`TraceChannel` "TraceTypeQuery3" :`DrawDebugType` "ForDuration"))
  (for (_array_element _array_index) _outhits
    (bind (_bblockinghit _binitialoverlap _time _distance _location _impactpoint _normal _impactnormal _physmat _hitactor _hitcomponent) (`GameplayStatics.BreakHitResult` _array_element))
    (`PrimitiveComponent.SetRenderCustomDepth` _hitcomponent true)
    (`KismetArrayLibrary.Array_Set` (`self.Hit Actor`) _array_index _hitactor true)))

(event `RotateLeftSelection`
  (params (Direction :type "Float (double-precision)"))
  (bind _returnvalue (> Direction 0.1))
  (for _array_element (`self.Hit Actor`)
    (if (not (`self.IsHorizontal`))
      (if _returnvalue
        (`self.HorizontalPositive` _array_element)
        (else
          (`self.HorizontalNegative` _array_element)))
      (elif _returnvalue
        (`self.VerticalNegative` _array_element)
        (else
          (`self.VerticalPositive` _array_element))))))

(event `HorizontalPositive`
  (params (ActorIn :type "Actor Object Reference"))
  (bind (_oldrotation_roll _oldrotation_pitch _oldrotation_yaw) (`KismetMathLibrary.BreakRotator` (`self.OldRotation`)))
  ;[0.5619 0.7927 1] HoPos
  (`|ExecutionSequence`
    (:`then_0`
      (set `self.OldRotation` (`self.K2_GetActorRotation` ActorIn)))
    (:`then_1`
      (set `self.NewRotation` (`KismetMathLibrary.MakeRotator` _oldrotation_roll _oldrotation_pitch (+ _oldrotation_yaw 90.0))))
    (:`then_2`
      (`self.K2_SetActorRelativeRotation` ActorIn (`KismetMathLibrary.RInterpTo` (`self.OldRotation`) (`self.NewRotation`) (`self.Delta Seconds`)) false false))))

(event `VerticalPositive`
  (params (ActorIn :type "Actor Object Reference"))
  (bind (_oldrotation_roll _oldrotation_pitch _oldrotation_yaw) (`KismetMathLibrary.BreakRotator` (`self.OldRotation`)))
  ;[0.5619 0.7927 1] VertPos
  (`|ExecutionSequence`
    (:`then_0`
      (set `self.OldRotation` (`self.K2_GetActorRotation` ActorIn)))
    (:`then_1`
      (set `self.NewRotation` (`KismetMathLibrary.MakeRotator` (+ _oldrotation_roll 90.0) _oldrotation_pitch _oldrotation_yaw)))
    (:`then_2`
      (`self.K2_SetActorRelativeRotation` ActorIn (`KismetMathLibrary.RInterpTo` (`self.OldRotation`) (`self.NewRotation`) (`self.Delta Seconds`)) false false))))

(event `HorizontalNegative`
  (params (ActorIn :type "Actor Object Reference"))
  (bind (_oldrotation_roll _oldrotation_pitch _oldrotation_yaw) (`KismetMathLibrary.BreakRotator` (`self.OldRotation`)))
  ;[0.961 1 0.5526] HoNeg
  (`|ExecutionSequence`
    (:`then_0`
      (set `self.OldRotation` (`self.K2_GetActorRotation` ActorIn)))
    (:`then_1`
      (set `self.NewRotation` (`KismetMathLibrary.MakeRotator` _oldrotation_roll _oldrotation_pitch (- _oldrotation_yaw 90.0))))
    (:`then_2`
      (`self.K2_SetActorRelativeRotation` ActorIn (`KismetMathLibrary.RInterpTo` (`self.OldRotation`) (`self.NewRotation`) (`self.Delta Seconds`)) false false))))

(event `VerticalNegative`
  (params (ActorIn :type "Actor Object Reference"))
  (bind (_oldrotation_roll _oldrotation_pitch _oldrotation_yaw) (`KismetMathLibrary.BreakRotator` (`self.OldRotation`)))
  ;[0.961 1 0.5526] VertNeg
  (`|ExecutionSequence`
    (:`then_0`
      (set `self.OldRotation` (`self.K2_GetActorRotation` ActorIn)))
    (:`then_1`
      (set `self.NewRotation` (`KismetMathLibrary.MakeRotator` (- _oldrotation_roll 90.0) _oldrotation_pitch _oldrotation_yaw)))
    (:`then_2`
      (`self.K2_SetActorRelativeRotation` ActorIn (`KismetMathLibrary.RInterpTo` (`self.OldRotation`) (`self.NewRotation`) (`self.Delta Seconds`)) false false))))

(event `TraceRight`
  ;[1 1 1] Traces
)

(event `EnhancedInput|/Game/FPPuzzleGame/Input/IA_Scroll`
  (params (ActionValue :type "Float (double-precision)") (ElapsedSeconds :type "Float (double-precision)") (TriggeredSeconds :type "Float (double-precision)") (InputAction :type "InputAction Object Reference" :default "/Game/FPPuzzleGame/Input/IA_Scroll.IA_Scroll"))
  (:`Started`
    (`KismetSystemLibrary.PrintString` (`KismetStringLibrary.Conv_DoubleToString` ActionValue))
    (`self.RotateLeftSelection` ActionValue)))

(event `EnhancedInput|/Game/FPPuzzleGame/Input/IA_Interact`
  (params (ActionValue :type Boolean) (ElapsedSeconds :type "Float (double-precision)") (TriggeredSeconds :type "Float (double-precision)") (InputAction :type "InputAction Object Reference" :default "/Game/FPPuzzleGame/Input/IA_Interact.IA_Interact"))
  (:`Started`
    (`/Engine/EditorBlueprintResources/StandardMacros.FlipFlop`
      (:`A`
        (set `self.IsHorizontal` true))
      (:`B`
        (set `self.IsHorizontal` false)))
    (`self.FlipSelection`)))

(event `EnhancedInput|/Game/FPPuzzleGame/Input/IA_Left`
  (params (ActionValue :type Boolean) (ElapsedSeconds :type "Float (double-precision)") (TriggeredSeconds :type "Float (double-precision)") (InputAction :type "InputAction Object Reference" :default "/Game/FPPuzzleGame/Input/IA_Left.IA_Left"))
  (:`Started`
    (set `self.PosInt` (- (`self.PosInt`) 1))
    (if (<= (`self.PosInt`) -1)
      (bind _output_get (set `self.PosInt` 2))
      (`self.MoveSelectah` _output_get)
      (else
        (`self.MoveSelectah` (`self.PosInt`))))))

(event `EnhancedInput|/Game/FPPuzzleGame/Input/IA_Right`
  (params (ActionValue :type Boolean) (ElapsedSeconds :type "Float (double-precision)") (TriggeredSeconds :type "Float (double-precision)") (InputAction :type "InputAction Object Reference" :default "/Game/FPPuzzleGame/Input/IA_Right.IA_Right"))
  (:`Started`
    (set `self.PosInt` (+ (`self.PosInt`) 1))
    (if (>= (`self.PosInt`) 3)
      (bind _output_get (set `self.PosInt` 0))
      (`self.MoveSelectah` _output_get)
      (else
        (`self.MoveSelectah` (`self.PosInt`))))))

(event `FlipSelection`
  (bind _traceholder (`self.TraceHolder`))
  ;[1 0.5368 0.4869] FlipSelectah
  (if (`self.IsHorizontal`)
    (`SceneComponent.K2_SetRelativeRotation` _traceholder (`KismetMathLibrary.MakeRotator` 90.0) false false)
    (else
      (`SceneComponent.K2_SetRelativeRotation` _traceholder (`KismetMathLibrary.MakeRotator` 0.0) false false)))
  (bind _output_get (set `self.PosInt` 1))
  (`self.MoveSelectah` _output_get))

(event `MoveSelectah`
  (params (PosInt :type Integer))
  (bind _traceholder (`self.TraceHolder`))
  (bind _traceholder_2 (`self.TraceHolder`))
  ;[1 0.403 0.4628] MoveSelectah
  (if (not (`self.IsHorizontal`))
    (switch `int` PosInt
      (:`0`
        (`SceneComponent.K2_SetRelativeLocation` _traceholder_2 (-278.0 0.0 -75.0) false false))
      (:`1`
        (`SceneComponent.K2_SetRelativeLocation` _traceholder_2 (-278.0 0.0 0.0) false false))
      (:`2`
        (`SceneComponent.K2_SetRelativeLocation` _traceholder_2 (-278.0 0.0 75.0) false false)))
    (else
      (switch `int` PosInt
        (:`0`
          (`SceneComponent.K2_SetRelativeLocation` _traceholder (-278.0 -75.0 0.0) false false))
        (:`1`
          (`SceneComponent.K2_SetRelativeLocation` _traceholder (-278.0 0.0 0.0) false false))
        (:`2`
          (`SceneComponent.K2_SetRelativeLocation` _traceholder (-278.0 75.0 0.0) false false))))))

(fn `UserConstructionScript`
  (`parent.UserConstructionScript`))