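; Possessable turnable-cylinder puzzle in which the player aligns three stacked cylinders that start at random yaws.
; Up/Down cycles the selection, highlighted through custom depth, and Left/Right rotates it.
; Releasing rotation flags cylinders within yaw tolerance; once all are flagged, timelines align and move them, then notify WinConActor.
; A height animation plays at BeginPlay and reverses when unpossessed after solving.
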(event `self.ReceiveBeginPlay`
  (`self.Inits`)
  (`KismetSystemLibrary.Delay` 0.2)
  (bind _returnvalue (`GameplayStatics.GetActorOfClass` "/Game/FPPuzzleGame/Blueprints/Player/BP_Player.BP_Player_C"))
  (set `self.PlayerRef` _returnvalue)
  (`self.OnPossessAnim`))

(event `/Game/FPPuzzleGame/Blueprints/Interfaces/BPI_Interact.Interact`
  (bind _playerref (`self.PlayerRef`))
  ;[1 1 1] Interact
  (set `/Game/FPPuzzleGame/Blueprints/Player/BP_Player.IsPlayingMiniGame` true _playerref)
  (`parent.Interact`)
  (set `/Game/FPPuzzleGame/Blueprints/Player/BP_Player.IsPlayingMiniGame` true _playerref)
  (set `self.SelectedInt` 0))

(event `self.ReceiveUnpossessed`
  (params (OldController :type "Controller Object Reference"))
  ;[1 1 1] Unpossessed
  (set `/Game/FPPuzzleGame/Blueprints/Player/BP_Player.IsPlayingMiniGame` false (`self.PlayerRef`))
  (`parent.ReceiveUnpossessed` OldController)
  (if (`self.IsActive`)
    (`self.OnUnpossessAnim`)))

(event `/Game/FPPuzzleGame/Blueprints/Interfaces/BPI_Interact.SetFocus`
  (params (IsFocused :type Boolean))
  ;[1 1 1] MarkFocused
  (if (not (`self.IsActive`))
    (`PrimitiveComponent.SetRenderCustomDepth` (`self.Meshes`) IsFocused)))

(event `FocusSelected`
  (bind _cylinder_low_top (`self.Cylinder_low_Top`))
  (bind _cylinder_low_middle (`self.Cylinder_low_Middle`))
  ;[1 1 1] MarkFocused
  (if (not (`self.IsActive`))
    (switch `int` (`self.SelectedInt`)
      (:`0`
        (`PrimitiveComponent.SetRenderCustomDepth` (`self.Cylinder_low_Bottom`) true)
        (`PrimitiveComponent.SetRenderCustomDepth` _cylinder_low_top false)
        (`PrimitiveComponent.SetRenderCustomDepth` _cylinder_low_middle false))
      (:`1`
        (`PrimitiveComponent.SetRenderCustomDepth` _cylinder_low_middle true)
        (`PrimitiveComponent.SetRenderCustomDepth` _cylinder_low_top false)
        (`PrimitiveComponent.SetRenderCustomDepth` (`self.Cylinder_low_Bottom`) false))
      (:`2`
        (`PrimitiveComponent.SetRenderCustomDepth` _cylinder_low_top true)
        (`PrimitiveComponent.SetRenderCustomDepth` _cylinder_low_middle false)
        (`PrimitiveComponent.SetRenderCustomDepth` (`self.Cylinder_low_Bottom`) false)))))

(event `TurnRenderDepthOff`
  (`PrimitiveComponent.SetRenderCustomDepth` (`self.Cylinder_low_Top`) false)
  (`PrimitiveComponent.SetRenderCustomDepth` (`self.Cylinder_low_Middle`) false)
  (`PrimitiveComponent.SetRenderCustomDepth` (`self.Cylinder_low_Bottom`) false))

(event `Inits`
  ;[1 1 1] Inits
  (`self.StartRandom`)
  (`self.FocusSelected`))

(event `StartRandom`
  (bind _returnvalue (`KismetMathLibrary.RandomFloatInRange` 40.0 300.0))
  ;[1 1 1] StartRandom
  (`SceneComponent.K2_SetWorldRotation` (`self.Cylinder_low_Bottom`) (`KismetMathLibrary.MakeRotator` 0.0 0.0 _returnvalue) false false)
  (`SceneComponent.K2_SetWorldRotation` (`self.Cylinder_low_Middle`) (`KismetMathLibrary.MakeRotator` 0.0 0.0 _returnvalue) false false)
  (`SceneComponent.K2_SetWorldRotation` (`self.Cylinder_low_Top`) (`KismetMathLibrary.MakeRotator` 0.0 0.0 _returnvalue) false false))

(event `CheckLockRotation`
  (bind (_relativerotation_roll _relativerotation_pitch _relativerotation_yaw) (`KismetMathLibrary.BreakRotator` (`SceneComponent.RelativeRotation` (`self.Cylinder_low_Top`))))
  (bind (_relativerotation_roll_2 _relativerotation_pitch_2 _relativerotation_yaw_2) (`KismetMathLibrary.BreakRotator` (`SceneComponent.RelativeRotation` (`self.Cylinder_low_Bottom`))))
  (bind (_relativerotation_roll_3 _relativerotation_pitch_3 _relativerotation_yaw_3) (`KismetMathLibrary.BreakRotator` (`SceneComponent.RelativeRotation` (`self.Cylinder_low_Middle`))))
  ;[1 0.58 0.1744] WinCon
  (`|ExecutionSequence`
    (:`then_0`
      (if (`KismetMathLibrary.InRange_FloatFloat` _relativerotation_yaw_2 -5.0 (`self.WinMaxRotation`))
        (set `self.AllowMoveBot` false)))
    (:`then_1`
      (if (`KismetMathLibrary.InRange_FloatFloat` _relativerotation_yaw_3 -5.0 (`self.WinMaxRotation`))
        (set `self.AllowMoveMid` false)))
    (:`then_2`
      (if (`KismetMathLibrary.InRange_FloatFloat` _relativerotation_yaw -5.0 (`self.WinMaxRotation`))
        (set `self.AllowMoveTop` false)))
    (:`then_3`
      (if (`self.AllowMoveTop`)
        _
        (elif (`self.AllowMoveMid`)
          _
          (elif (not (`self.AllowMoveBot`))
            (bind (_direction _alpha) (`Timeline|RotateToZero` :!via `PlayFromStart`)
              (:`Update`
                (set `self.AnimAlpha` _alpha)
                (`self.AllignCylinders`)))))))))

(event `TriggerWinCon`
  (bind _cylinder_low_middle (`self.Cylinder_low_Middle`))
  (bind _cylinder_low_top (`self.Cylinder_low_Top`))
  (bind _cylinder_low_bottom (`self.Cylinder_low_Bottom`))
  ;[0.3265 1 0.3458] TriggerWinCon
  (bind (_direction _alpha) (`Timeline|WinConAnim` :!via `PlayFromStart`)
    (:`Update`
      (`SceneComponent.K2_SetRelativeLocation` _cylinder_low_bottom (`KismetMathLibrary.VLerp` (`SceneComponent.RelativeLocation` _cylinder_low_bottom) (0.0 0.0 -50.0) _alpha) false false)
      (`SceneComponent.K2_SetRelativeLocation` _cylinder_low_middle (`KismetMathLibrary.VLerp` (`SceneComponent.RelativeLocation` _cylinder_low_middle) (0.0 0.0 -50.0) _alpha) false false)
      (`SceneComponent.K2_SetRelativeLocation` _cylinder_low_top (`KismetMathLibrary.VLerp` (`SceneComponent.RelativeLocation` _cylinder_low_top) (0.0 0.0 -50.0) _alpha) false false))
    (:`Finished`
      (message `/Game/FPPuzzleGame/Blueprints/Interfaces/BPI_Puzzle.PuzzleSolved` (`self.WinConActor`))
      (set `self.IsActive` true))))

(event `EnhancedInput|/Game/FPPuzzleGame/Input/IA_Right`
  (params (ActionValue :type Boolean) (ElapsedSeconds :type "Float (double-precision)") (TriggeredSeconds :type "Float (double-precision)") (InputAction :type "InputAction Object Reference" :default "/Game/FPPuzzleGame/Input/IA_Right.IA_Right"))
  (bind _returnvalue (* TriggeredSeconds (`self.MoveFloat`)))
  ;[0.657 0.3538 1] Controls
  (:`Triggered`
    (switch `int` (`self.SelectedInt`)
      (:`0`
        (`SceneComponent.K2_AddWorldRotation` (`self.Cylinder_low_Bottom`) (`KismetMathLibrary.MakeRotator` 0.0 0.0 _returnvalue) false false))
      (:`1`
        (`SceneComponent.K2_AddWorldRotation` (`self.Cylinder_low_Middle`) (`KismetMathLibrary.MakeRotator` 0.0 0.0 _returnvalue) false false))
      (:`2`
        (`SceneComponent.K2_AddWorldRotation` (`self.Cylinder_low_Top`) (`KismetMathLibrary.MakeRotator` 0.0 0.0 _returnvalue) false false))))
  (:`Completed`
    (`self.CheckLockRotation`)))

(event `EnhancedInput|/Game/FPPuzzleGame/Input/IA_Left`
  (params (ActionValue :type Boolean) (ElapsedSeconds :type "Float (double-precision)") (TriggeredSeconds :type "Float (double-precision)") (InputAction :type "InputAction Object Reference" :default "/Game/FPPuzzleGame/Input/IA_Left.IA_Left"))
  (bind _returnvalue (* TriggeredSeconds (* (`self.MoveFloat`) -1.0)))
  ;[0.657 0.3538 1] Controls
  (:`Triggered`
    (switch `int` (`self.SelectedInt`)
      (:`0`
        (`SceneComponent.K2_AddWorldRotation` (`self.Cylinder_low_Bottom`) (`KismetMathLibrary.MakeRotator` 0.0 0.0 _returnvalue) false false))
      (:`1`
        (`SceneComponent.K2_AddWorldRotation` (`self.Cylinder_low_Middle`) (`KismetMathLibrary.MakeRotator` 0.0 0.0 _returnvalue) false false))
      (:`2`
        (`SceneComponent.K2_AddWorldRotation` (`self.Cylinder_low_Top`) (`KismetMathLibrary.MakeRotator` 0.0 0.0 _returnvalue) false false))))
  (:`Completed`
    (`self.CheckLockRotation`)))

(event `EnhancedInput|/Game/FPPuzzleGame/Input/IA_Up`
  (params (ActionValue :type Boolean) (ElapsedSeconds :type "Float (double-precision)") (TriggeredSeconds :type "Float (double-precision)") (InputAction :type "InputAction Object Reference" :default "/Game/FPPuzzleGame/Input/IA_Up.IA_Up"))
  ;[0.657 0.3538 1] Controls
  (:`Started`
    (bind _output_get (set `self.SelectedInt` (+ (`self.SelectedInt`) 1)))
    (if (>= _output_get 3)
      (set `self.SelectedInt` 0))
    (`self.FocusSelected`)))

(event `EnhancedInput|/Game/FPPuzzleGame/Input/IA_Down`
  (params (ActionValue :type Boolean) (ElapsedSeconds :type "Float (double-precision)") (TriggeredSeconds :type "Float (double-precision)") (InputAction :type "InputAction Object Reference" :default "/Game/FPPuzzleGame/Input/IA_Down.IA_Down"))
  ;[0.657 0.3538 1] Controls
  (:`Started`
    (bind _output_get (set `self.SelectedInt` (- (`self.SelectedInt`) 1)))
    (if (<= _output_get -1)
      (set `self.SelectedInt` 2))
    (`self.FocusSelected`)))

(event `AllignCylinders`
  ;[1 0.58 0.1744] WinCon
  (`SceneComponent.K2_SetWorldRotation` (`self.Cylinder_low_Bottom`) (`KismetMathLibrary.RLerp` (`SceneComponent.K2_GetComponentRotation` (`self.Cylinder_low_Bottom`)) (struct) (`self.AnimAlpha`) true) false false)
  (`SceneComponent.K2_SetWorldRotation` (`self.Cylinder_low_Middle`) (`KismetMathLibrary.RLerp` (`SceneComponent.K2_GetComponentRotation` (`self.Cylinder_low_Middle`)) (struct) (`self.AnimAlpha`) true) false false)
  (`SceneComponent.K2_SetWorldRotation` (`self.Cylinder_low_Top`) (`KismetMathLibrary.RLerp` (`SceneComponent.K2_GetComponentRotation` (`self.Cylinder_low_Top`)) (struct) (`self.AnimAlpha`) true) false false)
  (`self.TriggerWinCon`)
  (`self.TurnRenderDepthOff`))

(event `OnPossessAnim`
  ;[1 0.2572 0.5326] Un|Posses Animation
  (`/Engine/EditorBlueprintResources/StandardMacros.DoOnce` false
    (:`Completed`
      (bind (_direction _alpha) (`Timeline|PossessAnim` :!via `PlayFromStart` :!label _label)
        (:`Update`
          (set `self.PossessAnimalpha` _alpha)
          (switch `ETimelineDirection` _direction
            (:`Forward`
              (`self.PossessForward`))
            (:`Backward`
              (`self.PossessBackwards`))))
        (:`Finished`
          (`self.FocusSelected`)
          (`/Engine/EditorBlueprintResources/StandardMacros.DoOnce` false
            (:`Completed`
              (`KismetSystemLibrary.Delay` 5.0))))))))

(event `OnUnpossessAnim`
  ;[1 0.2572 0.5326] Un|Posses Animation
  (`/Engine/EditorBlueprintResources/StandardMacros.DoOnce` false
    (:`Completed`
      (goto _label :!via `ReverseFromEnd`))))

(event `PossessBackwards`
  (bind _cylinder_low_middle (`self.Cylinder_low_Middle`))
  (bind _cylinder_low_top (`self.Cylinder_low_Top`))
  (bind _cylinder_low_bottom (`self.Cylinder_low_Bottom`))
  (bind (_relativelocation_x _relativelocation_y _relativelocation_z) (`KismetMathLibrary.BreakVector` (`SceneComponent.RelativeLocation` _cylinder_low_bottom)))
  (bind (_relativelocation_x_2 _relativelocation_y_2 _relativelocation_z_2) (`KismetMathLibrary.BreakVector` (`SceneComponent.RelativeLocation` _cylinder_low_top)))
  (bind (_relativelocation_x_3 _relativelocation_y_3 _relativelocation_z_3) (`KismetMathLibrary.BreakVector` (`SceneComponent.RelativeLocation` _cylinder_low_middle)))
  ;[1 0.2572 0.5326] Un|Posses Animation
  (`SceneComponent.K2_SetRelativeLocation` (`self.Cylinder_low_Bottom`) (`KismetMathLibrary.VLerp` (`SceneComponent.RelativeLocation` _cylinder_low_bottom) (`KismetMathLibrary.MakeVector` _relativelocation_x _relativelocation_y (- _relativelocation_z (`self.HeightBot`))) (`self.PossessAnimalpha`)) false false)
  (`SceneComponent.K2_SetRelativeLocation` (`self.Cylinder_low_Top`) (`KismetMathLibrary.VLerp` (`SceneComponent.RelativeLocation` _cylinder_low_top) (`KismetMathLibrary.MakeVector` _relativelocation_x_2 _relativelocation_y_2 (- _relativelocation_z_2 (`self.HeightTop`))) (`self.PossessAnimalpha`)) false false)
  (`SceneComponent.K2_SetRelativeLocation` (`self.Cylinder_low_Middle`) (`KismetMathLibrary.VLerp` (`SceneComponent.RelativeLocation` _cylinder_low_middle) (`KismetMathLibrary.MakeVector` _relativelocation_x_3 _relativelocation_y_3 (- _relativelocation_z_3 (`self.HeightMid`))) (`self.PossessAnimalpha`)) false false))

(event `PossessForward`
  (bind _cylinder_low_bottom (`self.Cylinder_low_Bottom`))
  (bind _cylinder_low_middle (`self.Cylinder_low_Middle`))
  (bind _cylinder_low_top (`self.Cylinder_low_Top`))
  (bind (_relativelocation_x _relativelocation_y _relativelocation_z) (`KismetMathLibrary.BreakVector` (`SceneComponent.RelativeLocation` _cylinder_low_bottom)))
  (bind (_relativelocation_x_2 _relativelocation_y_2 _relativelocation_z_2) (`KismetMathLibrary.BreakVector` (`SceneComponent.RelativeLocation` _cylinder_low_top)))
  (bind (_relativelocation_x_3 _relativelocation_y_3 _relativelocation_z_3) (`KismetMathLibrary.BreakVector` (`SceneComponent.RelativeLocation` _cylinder_low_middle)))
  ;[1 0.2572 0.5326] Un|Posses Animation
  (`SceneComponent.K2_SetRelativeLocation` (`self.Cylinder_low_Bottom`) (`KismetMathLibrary.VLerp` (`SceneComponent.RelativeLocation` _cylinder_low_bottom) (`KismetMathLibrary.MakeVector` _relativelocation_x _relativelocation_y (+ _relativelocation_z (`self.HeightBot`))) (`self.PossessAnimalpha`)) false false)
  (`SceneComponent.K2_SetRelativeLocation` (`self.Cylinder_low_Top`) (`KismetMathLibrary.VLerp` (`SceneComponent.RelativeLocation` _cylinder_low_top) (`KismetMathLibrary.MakeVector` _relativelocation_x_2 _relativelocation_y_2 (+ _relativelocation_z_2 (`self.HeightTop`))) (`self.PossessAnimalpha`)) false false)
  (`SceneComponent.K2_SetRelativeLocation` (`self.Cylinder_low_Middle`) (`KismetMathLibrary.VLerp` (`SceneComponent.RelativeLocation` _cylinder_low_middle) (`KismetMathLibrary.MakeVector` _relativelocation_x_3 _relativelocation_y_3 (+ _relativelocation_z_3 (`self.HeightMid`))) (`self.PossessAnimalpha`)) false false))

(fn `UserConstructionScript`
  (`parent.UserConstructionScript`))