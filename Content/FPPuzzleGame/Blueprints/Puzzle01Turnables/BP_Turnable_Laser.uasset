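; BP_Turnable_Laser is a possessable puzzle piece whose Mid component the player rotates around the yaw axis.
; On BeginPlay it gives Mid a random yaw and enables its custom depth rendering.
; Left and right Enhanced Input actions rotate Mid, scaled by triggered seconds and MoveFloat.
; Interact and Unpossessed extend parent logic, but the possess animation, win trigger and up/down inputs are empty, with older animation and selection logic left disconnected.
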(event `self.ReceiveBeginPlay`
  (`self.Inits`))

(event `self.Interact`
  ;[1 1 1] Interact
  (`parent.Interact`)
  (`self.OnPossessAnim`))

(event `self.ReceiveUnpossessed`
  (params (OldController :type "Controller Object Reference"))
  ;[1 1 1] Unpossessed
  (`parent.ReceiveUnpossessed` OldController)
  (`self.OnPossessAnim`))

(event `FocusSelected`
  ;[1 1 1] MarkFocused
  (`PrimitiveComponent.SetRenderCustomDepth` (`self.Mid`) true))

(event `Inits`
  ;[1 1 1] Inits
  (`self.StartRandom`)
  (`self.FocusSelected`))

(event `StartRandom`
  ;[1 1 1] StartRandom
  (`SceneComponent.K2_SetWorldRotation` (`self.Mid`) (`KismetMathLibrary.MakeRotator` 0.0 0.0 (`KismetMathLibrary.RandomFloatInRange` 40.0 300.0)) false false))

(event `TriggerWinCon`
  ;[0.3265 1 0.3458] TriggerWinCon
)

(event `EnhancedInput|/Game/FPPuzzleGame/Input/IA_Right`
  (params (ActionValue :type Boolean) (ElapsedSeconds :type "Float (double-precision)") (TriggeredSeconds :type "Float (double-precision)") (InputAction :type "InputAction Object Reference" :default "/Game/FPPuzzleGame/Input/IA_Right.IA_Right"))
  ;[0.657 0.3538 1] Controls
  (:`Triggered`
    (if true
      (`SceneComponent.K2_AddWorldRotation` (`self.Mid`) (`KismetMathLibrary.MakeRotator` 0.0 0.0 (* TriggeredSeconds (`self.MoveFloat`))) false false))))

(event `EnhancedInput|/Game/FPPuzzleGame/Input/IA_Left`
  (params (ActionValue :type Boolean) (ElapsedSeconds :type "Float (double-precision)") (TriggeredSeconds :type "Float (double-precision)") (InputAction :type "InputAction Object Reference" :default "/Game/FPPuzzleGame/Input/IA_Left.IA_Left"))
  ;[0.657 0.3538 1] Controls
  (:`Triggered`
    (if true
      (`SceneComponent.K2_AddWorldRotation` (`self.Mid`) (`KismetMathLibrary.MakeRotator` 0.0 0.0 (* TriggeredSeconds (* (`self.MoveFloat`) -1.0))) false false))))

(event `EnhancedInput|/Game/FPPuzzleGame/Input/IA_Up`
  (params (ActionValue :type Boolean) (ElapsedSeconds :type "Float (double-precision)") (TriggeredSeconds :type "Float (double-precision)") (InputAction :type "InputAction Object Reference" :default "/Game/FPPuzzleGame/Input/IA_Up.IA_Up"))
  ;[0.657 0.3538 1] Controls
)

(event `EnhancedInput|/Game/FPPuzzleGame/Input/IA_Down`
  (params (ActionValue :type Boolean) (ElapsedSeconds :type "Float (double-precision)") (TriggeredSeconds :type "Float (double-precision)") (InputAction :type "InputAction Object Reference" :default "/Game/FPPuzzleGame/Input/IA_Down.IA_Down"))
  ;[0.657 0.3538 1] Controls
)

(event `OnPossessAnim`
  ;[1 0.2572 0.5326] Un|Posses Animation
)

(event `PossessForward`
  (bind _mid (`self.Mid`))
  (bind (_relativelocation_x _relativelocation_y _relativelocation_z) (`KismetMathLibrary.BreakVector` (`SceneComponent.RelativeLocation` _mid)))
  ;[1 0.2572 0.5326] Un|Posses Animation
  (`SceneComponent.K2_SetRelativeLocation` _mid (`KismetMathLibrary.VLerp` (`SceneComponent.RelativeLocation` _mid) (`KismetMathLibrary.MakeVector` _relativelocation_x _relativelocation_y (+ _relativelocation_z (`self.HeightMid`))) (`self.PossessAnimalpha`)) false false))

(event `PossessBackwards`
  (bind _mid (`self.Mid`))
  (bind (_relativelocation_x _relativelocation_y _relativelocation_z) (`KismetMathLibrary.BreakVector` (`SceneComponent.RelativeLocation` _mid)))
  ;[1 0.2572 0.5326] Un|Posses Animation
  (`SceneComponent.K2_SetRelativeLocation` _mid (`KismetMathLibrary.VLerp` (`SceneComponent.RelativeLocation` _mid) (`KismetMathLibrary.MakeVector` _relativelocation_x _relativelocation_y (- _relativelocation_z 2.0)) (`self.PossessAnimalpha`)) false false))

(fn `UserConstructionScript`
  (`parent.UserConstructionScript`))