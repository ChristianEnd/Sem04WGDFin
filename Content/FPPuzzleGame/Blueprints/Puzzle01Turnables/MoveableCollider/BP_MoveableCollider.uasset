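; Movable selection box for a turnable minigame puzzle, picking groups of BPI_MiniGameTurnable pieces to rotate.
; The box jumps between marker positions along a horizontal or vertical axis, and flipping re-centers and rotates it.
; Overlaps fill ActiveSelection, changing materials at nine pieces and reverting on end overlap.
; Turn rotates selected pieces on yaw or roll through timeline-driven RInterpTo toward a moving 90-degree offset, with CanInput blocking overlapping actions.
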(event `self.ReceiveBeginPlay`
  ;[1 1 1] Start
  (set `self.StartLocation` (`SceneComponent.K2_GetComponentLocation` (`self.Box`))))

(event `MoveDown/Lef`
  (params (PositionInt :type Integer))
  ;[1 1 1] NewLeft
  (`|ExecutionSequence`
    (:`then_0`
      (`self.ClearActiveSelection`))
    (:`then_1`
      (if (`self.CanInput`)
        (switch `string` (`KismetStringLibrary.Conv_IntToString` PositionInt)
          (:`-1`
            (if (`self.IsHorizontal`)
              (`SceneComponent.K2_SetWorldLocation` (`self.Box`) (`SceneComponent.K2_GetComponentLocation` (`self.H-1`)) false false)
              (else
                (`SceneComponent.K2_SetWorldLocation` (`self.Box`) (`SceneComponent.K2_GetComponentLocation` (`self.V-1`)) false false))))
          (:`0`
            (if (`self.IsHorizontal`)
              _
              (else
                _))
            (`SceneComponent.K2_SetWorldLocation` (`self.Box`) (`SceneComponent.K2_GetComponentLocation` (`self.0`)) false false))
          (:`1`
            (if (`self.IsHorizontal`)
              (`SceneComponent.K2_SetWorldLocation` (`self.Box`) (`SceneComponent.K2_GetComponentLocation` (`self.H1`)) false false)
              (else
                (`SceneComponent.K2_SetWorldLocation` (`self.Box`) (`SceneComponent.K2_GetComponentLocation` (`self.V1`)) false false)))))))))

(event `MoveUp/Right`
  (params (PositionInt :type Integer))
  ;[1 1 1] NewRight
  (`|ExecutionSequence`
    (:`then_0`
      (`self.ClearActiveSelection`))
    (:`then_1`
      (if (`self.CanInput`)
        (switch `string` (`KismetStringLibrary.Conv_IntToString` PositionInt)
          (:`-1`
            (if (`self.IsHorizontal`)
              (`SceneComponent.K2_SetWorldLocation` (`self.Box`) (`SceneComponent.K2_GetComponentLocation` (`self.H-1`)) false false)
              (else
                (`SceneComponent.K2_SetWorldLocation` (`self.Box`) (`SceneComponent.K2_GetComponentLocation` (`self.V-1`)) false false))))
          (:`0`
            (if (`self.IsHorizontal`)
              _
              (else
                _))
            (`SceneComponent.K2_SetWorldLocation` (`self.Box`) (`SceneComponent.K2_GetComponentLocation` (`self.0`)) false false))
          (:`1`
            (if (`self.IsHorizontal`)
              (`SceneComponent.K2_SetWorldLocation` (`self.Box`) (`SceneComponent.K2_GetComponentLocation` (`self.H1`)) false false)
              (else
                (`SceneComponent.K2_SetWorldLocation` (`self.Box`) (`SceneComponent.K2_GetComponentLocation` (`self.V1`)) false false)))))))))

(event `FlipIt`
  (params (IsHorizontal :type Boolean))
  ;[1 0 0.1641] FlipTheCollider
  (if (`self.CanInput`)
    (`|ExecutionSequence`
      (:`then_0`
        (if (not (`self.IsHorizontal`))
          (set `self.CanInput` false)
          (`SceneComponent.K2_SetWorldLocation` (`self.Box`) (`SceneComponent.K2_GetComponentLocation` (`self.H1`)) false false)
          (`KismetSystemLibrary.Delay` 0.5)
          (`SceneComponent.K2_SetWorldLocation` (`self.Box`) (`SceneComponent.K2_GetComponentLocation` (`self.0`)) false false)
          (else
            (set `self.CanInput` false)
            (`SceneComponent.K2_SetWorldLocation` (`self.Box`) (`SceneComponent.K2_GetComponentLocation` (`self.V1`)) false false)
            (`KismetSystemLibrary.Delay` 0.5)
            (`SceneComponent.K2_SetWorldLocation` (`self.Box`) (`SceneComponent.K2_GetComponentLocation` (`self.0`)) false false))))
      (:`then_1`
        (set `self.Position Int` 0)
        (`self.RotateSelecta`)))))

(event `self.ReceiveTick`
  (params (DeltaSeconds :type "Float (single-precision)"))
  (set `self.Delta Seconds` DeltaSeconds))

(event `RotateSelecta`
  (bind _box (`self.Box`))
  ;[0.7578 1 0] RotateTheCollider
  (`|ExecutionSequence`
    (:`then_0`
      (`/Engine/EditorBlueprintResources/StandardMacros.FlipFlop`
        (:`A`
          (set `self.IsHorizontal` false)
          (`SceneComponent.K2_SetRelativeRotation` _box (`KismetMathLibrary.MakeRotator` 0.0 90.0) false false))
        (:`B`
          (set `self.IsHorizontal` true)
          (`SceneComponent.K2_SetRelativeRotation` _box (`KismetMathLibrary.MakeRotator` 0.0) false false))))
    (:`then_1`
      (set `self.CanInput` true))))

(event `self.Box.OnComponentBeginOverlap`
  (params (OverlappedComponent :type "PrimitiveComponent Object Reference") (OtherActor :type "Actor Object Reference") (OtherComp :type "PrimitiveComponent Object Reference") (OtherBodyIndex :type Integer) (bFromSweep :type Boolean) (SweepResult :type "HitResult Structure (by ref)"))
  (bind _indexcount (`self.IndexCount`))
  ;[0.2656 1 0] AddToArray
  (if (`KismetSystemLibrary.DoesImplementInterface` OtherActor "/Game/FPPuzzleGame/Blueprints/Interfaces/BPI_MiniGameTurnable.BPI_MiniGameTurnable_C")
    (`KismetArrayLibrary.Array_Set` (`self.ActiveSelection`) _indexcount OtherActor true)
    (set `self.IndexCount` (+ _indexcount 1))
    (if (== _indexcount 9)
      (set `self.IndexCount` 0)
      (`self.ChangeMatSelected`))))

(event `ClearActiveSelection`
  ;[1 0.2083 0.2083] ClearArray
  (`KismetArrayLibrary.Array_Clear` (`self.ActiveSelection`)))

(event `self.Box.OnComponentEndOverlap`
  (params (OverlappedComponent :type "PrimitiveComponent Object Reference") (OtherActor :type "Actor Object Reference") (OtherComp :type "PrimitiveComponent Object Reference") (OtherBodyIndex :type Integer))
  ;[0.2656 1 0] AddToArray
  (if (`KismetSystemLibrary.DoesImplementInterface` OtherActor "/Game/FPPuzzleGame/Blueprints/Interfaces/BPI_MiniGameTurnable.BPI_MiniGameTurnable_C")
    (`self.ChangeBackMaterial`)))

(event `ChangeMatSelected`
  (bind _activeselection (`self.ActiveSelection`))
  ;[0.2656 1 0] AddToArray
  (for (_ _array_index) _activeselection
    (bind _returnvalue (`self.GetComponentByClass` (`|GetArrayItem` _activeselection _array_index) "/Script/Engine.MeshComponent"))
    (`PrimitiveComponent.SetMaterial` _returnvalue 0 "/Game/FPPuzzleGame/Materials/General/M_MI_E_Green.M_MI_E_Green")
    (`PrimitiveComponent.SetMaterial` _returnvalue 0 "/Game/FPPuzzleGame/Materials/General/M_.M_")))

(event `ActivateInput`
  ;[1 1 1] Act/Dis Input
  (`self.EnableInput` (`GameplayStatics.GetPlayerPawn` 0) (`GameplayStatics.GetPlayerController` 0)))

(event `DeactivateInput`
  ;[1 1 1] Act/Dis Input
  (`self.DisableInput` (`GameplayStatics.GetPlayerPawn` 0) (`GameplayStatics.GetPlayerController` 0)))

(event `ChangeBackMaterial`
  (bind _activeselection (`self.ActiveSelection`))
  ;[1 0.5848 0.3188] RevertMat
  (for (_ _array_index) _activeselection
    (bind _returnvalue (`self.GetComponentByClass` (`|GetArrayItem` _activeselection _array_index) "/Script/Engine.MeshComponent"))
    (`PrimitiveComponent.SetMaterial` _returnvalue 0 "/Game/FPPuzzleGame/Materials/General/M_MI_E_Green.M_MI_E_Green")
    (`PrimitiveComponent.SetMaterial` _returnvalue 0 "/Game/StarterContent/Materials/M_Brick_Clay_Old.M_Brick_Clay_Old")))

(event `ComponentMaterialChange`
  ;[1 0.6941 0.4031] ChangeMat
  (for _array_element (`self.Other Comp`)
    (`PrimitiveComponent.SetMaterial` _array_element 0 "/Game/FPPuzzleGame/Materials/General/M_MI_E_Green.M_MI_E_Green")
    (`PrimitiveComponent.SetMaterial` _array_element 0 "/Game/FPPuzzleGame/Materials/General/M_.M_")))

(event `Turn`
  (params (TurnDirection :type "Float (double-precision)"))
  (bind (_activeactorrotation_roll _activeactorrotation_pitch _activeactorrotation_yaw) (`KismetMathLibrary.BreakRotator` (`self.ActiveActorRotation`)))
  (bind (_activeactorrotation_roll_2 _activeactorrotation_pitch_2 _activeactorrotation_yaw_2) (`KismetMathLibrary.BreakRotator` (`self.ActiveActorRotation`)))
  (bind (_activeactorrotation_roll_3 _activeactorrotation_pitch_3 _activeactorrotation_yaw_3) (`KismetMathLibrary.BreakRotator` (`self.ActiveActorRotation`)))
  (bind (_activeactorrotation_roll_4 _activeactorrotation_pitch_4 _activeactorrotation_yaw_4) (`KismetMathLibrary.BreakRotator` (`self.ActiveActorRotation`)))
  ;[1 0.2487 0.8122] Rotation
  (if (`self.CanInput`)
    (if (`self.IsHorizontal`)
      (if (> TurnDirection 0.0)
        (set `self.CanInput` false)
        (bind (_direction _alpha) (`Timeline|Timeline_2` :!via `PlayFromStart`)
          (:`Update`
            (set `self.Anim_Alpha` _alpha)
            (for _array_element (`self.ActiveSelection`)
              (`|ExecutionSequence`
                (:`then_0`
                  (bind _output_get (set `self.ActiveArrayElement` _array_element))
                  (set `self.ActiveActorRotation` (`self.K2_GetActorRotation` _output_get)))
                (:`then_1`
                  (set `self.ActiveActorAddedRotation` (`KismetMathLibrary.MakeRotator` _activeactorrotation_roll_2 _activeactorrotation_pitch_2 (- _activeactorrotation_yaw_2 90.0))))
                (:`then_2`
                  (`SceneComponent.K2_SetWorldRotation` (`Actor.RootComponent` (`self.ActiveArrayElement`)) (`KismetMathLibrary.RInterpTo` (`self.ActiveActorRotation`) (`self.ActiveActorAddedRotation`) (`self.Delta Seconds`) (`self.Interp Speed`)) false false)))))
          (:`Finished`
            (set `self.CanInput` true)))
        (else
          (set `self.CanInput` false)
          (bind (_direction_2 _alpha_2) (`Timeline|Timeline_1` :!via `PlayFromStart`)
            (:`Update`
              (set `self.Anim_Alpha` _alpha_2)
              (for _array_element_2 (`self.ActiveSelection`)
                (`|ExecutionSequence`
                  (:`then_0`
                    (bind _output_get_2 (set `self.ActiveArrayElement` _array_element_2))
                    (set `self.ActiveActorRotation` (`self.K2_GetActorRotation` _output_get_2)))
                  (:`then_1`
                    (set `self.ActiveActorAddedRotation` (`KismetMathLibrary.MakeRotator` _activeactorrotation_roll_4 _activeactorrotation_pitch_4 (+ _activeactorrotation_yaw_4 90.0))))
                  (:`then_2`
                    (`SceneComponent.K2_SetWorldRotation` (`Actor.RootComponent` (`self.ActiveArrayElement`)) (`KismetMathLibrary.RInterpTo` (`self.ActiveActorRotation`) (`self.ActiveActorAddedRotation`) (`self.Delta Seconds`) (`self.Interp Speed`)) false false)))))
            (:`Finished`
              (set `self.CanInput` true)))))
      (elif (> TurnDirection 0.0)
        (set `self.CanInput` false)
        (bind (_direction_3 _alpha_3) (`Timeline|Timeline_0` :!via `PlayFromStart`)
          (:`Update`
            (set `self.Anim_Alpha` _alpha_3)
            (for _array_element_3 (`self.ActiveSelection`)
              (`|ExecutionSequence`
                (:`then_0`
                  (bind _output_get_3 (set `self.ActiveArrayElement` _array_element_3))
                  (set `self.ActiveActorRotation` (`self.K2_GetActorRotation` _output_get_3)))
                (:`then_1`
                  (set `self.ActiveActorAddedRotation` (`KismetMathLibrary.MakeRotator` (- _activeactorrotation_roll 90.0) _activeactorrotation_pitch _activeactorrotation_yaw)))
                (:`then_2`
                  (`SceneComponent.K2_SetWorldRotation` (`Actor.RootComponent` (`self.ActiveArrayElement`)) (`KismetMathLibrary.RInterpTo` (`self.ActiveActorRotation`) (`self.ActiveActorAddedRotation`) (`self.Delta Seconds`) (`self.Interp Speed`)) false false)))))
          (:`Finished`
            (set `self.CanInput` true)))
        (else
          (set `self.CanInput` false)
          (bind (_direction_4 _alpha_4) (`Timeline|Timeline` :!via `PlayFromStart`)
            (:`Update`
              (set `self.Anim_Alpha` _alpha_4)
              (for _array_element_4 (`self.ActiveSelection`)
                (`|ExecutionSequence`
                  (:`then_0`
                    (bind _output_get_4 (set `self.ActiveArrayElement` _array_element_4))
                    (set `self.ActiveActorRotation` (`self.K2_GetActorRotation` _output_get_4)))
                  (:`then_1`
                    (set `self.ActiveActorAddedRotation` (`KismetMathLibrary.MakeRotator` (+ _activeactorrotation_roll_3 90.0) _activeactorrotation_pitch_3 _activeactorrotation_yaw_3)))
                  (:`then_2`
                    (`SceneComponent.K2_SetWorldRotation` (`Actor.RootComponent` (`self.ActiveArrayElement`)) (`KismetMathLibrary.RInterpTo` (`self.ActiveActorRotation`) (`self.ActiveActorAddedRotation`) (`self.Delta Seconds`) (`self.Interp Speed`)) false false)))))
            (:`Finished`
              (set `self.CanInput` true))))))))

(fn `UserConstructionScript`)