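; Interactable sliding-puzzle cube that moves one step into a free neighbouring space on a vertical X/Z plane.
; On Interact, if movement is allowed, four visibility line traces probe for blockers, and the last unblocked direction sets MoveDirectionInt.
; DirectionLogic then teleports the root by MoveDistance and saves the new location.
; BeginPlay scales move and trace distances by owner Z scale, and focus toggles a custom depth highlight.
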(event `DirectionLogic`
  (switch `int` (`self.MoveDirectionInt`)
    (:`0`
      (`KismetSystemLibrary.PrintString` "ICHKANN MICH DOCH NICHT BEWEGEN"))
    (:`1`
      (`self.MoveToNorth`)
      (set `self.MoveDirectionInt` 5 :!label _label))
    (:`2`
      (`self.MoveToSouth`)
      (goto _label))
    (:`3`
      (`self.MoveToWest`)
      (goto _label))
    (:`4`
      (`self.MoveToEast`)
      (goto _label))))

(event `SafeLocation`
  (set `self.StartTransform` (`self.K2_GetActorLocation` self)))

(event `MoveToEast`
  (bind (_starttransform_x _starttransform_y _starttransform_z) (`KismetMathLibrary.BreakVector` (`self.StartTransform`)))
  (`SceneComponent.K2_SetWorldLocation` (`self.DefaultSceneRoot`) (`KismetMathLibrary.MakeVector` (+ _starttransform_x (`self.MoveDistance`)) _starttransform_y _starttransform_z) false false)
  (`self.SafeLocation`))

(event `MoveToNorth`
  (bind (_starttransform_x _starttransform_y _starttransform_z) (`KismetMathLibrary.BreakVector` (`self.StartTransform`)))
  (`SceneComponent.K2_SetWorldLocation` (`self.DefaultSceneRoot`) (`KismetMathLibrary.MakeVector` _starttransform_x _starttransform_y (+ _starttransform_z (`self.MoveDistance`))) false false)
  (`self.SafeLocation`))

(event `MoveToWest`
  (bind (_starttransform_x _starttransform_y _starttransform_z) (`KismetMathLibrary.BreakVector` (`self.StartTransform`)))
  (`SceneComponent.K2_SetWorldLocation` (`self.DefaultSceneRoot`) (`KismetMathLibrary.MakeVector` (- _starttransform_x (`self.MoveDistance`)) _starttransform_y _starttransform_z) false false)
  (`self.SafeLocation`))

(event `MoveToSouth`
  (bind (_starttransform_x _starttransform_y _starttransform_z) (`KismetMathLibrary.BreakVector` (`self.StartTransform`)))
  (`SceneComponent.K2_SetWorldLocation` (`self.DefaultSceneRoot`) (`KismetMathLibrary.MakeVector` _starttransform_x _starttransform_y (- _starttransform_z (`self.MoveDistance`))) false false)
  (`self.SafeLocation`))

(event `self.SetFocus`
  (params (IsFocused :type Boolean))
  ;[1 0.9429 0.2055] SetFocus
  (`PrimitiveComponent.SetRenderCustomDepth` (`self.MoveableCube`) IsFocused))

(event `self.Interact`
  (if (`self.GeneralMoveAllowed`)
    (`|ExecutionSequence`
      (:`then_0`
        (`self.StartTraces`)))))

(event `self.ReceiveBeginPlay`
  (`self.SafeLocation`)
  (`self.SetDynamicMoveDistance`))

(event `SetMoveAllowed`
  (set `self.GeneralMoveAllowed` true))

(event `SetDynamicMoveDistance`
  (bind _returnvalue (`self.GetOwner` self))
  (bind (_returnvalue_x _returnvalue_y _returnvalue_z) (`KismetMathLibrary.BreakVector` (`self.GetActorScale3D` _returnvalue)))
  ;[1 1 1] SetDynamicMoveDistanceByScale
  (`/Engine/EditorBlueprintResources/StandardMacros.IsValid` _returnvalue
    (:`Is Valid`
      (set `self.MoveDistance` (* _returnvalue_z (`self.MoveDistance`)))
      (set `self.TracDistance` (* _returnvalue_z (`self.TracDistance`))))))

(event `SetMoveAmountAndTraceLength`
  (bind (_returnvalue_x _returnvalue_y _returnvalue_z) (`KismetMathLibrary.BreakVector` (`self.K2_GetActorLocation`)))
  (bind (_out_hit_impact_point_x _out_hit_impact_point_y _out_hit_impact_point_z) (`KismetMathLibrary.BreakVector` (`self.Out Hit Impact Point`)))
  (`self.StartTraces`)
  (set `self.TracDistance` (- _returnvalue_z _out_hit_impact_point_z)))

(event `StartTraces`
  (bind _moveablecube (`self.MoveableCube`))
  (bind _moveablecube_2 (`self.MoveableCube`))
  (bind _moveablecube_3 (`self.MoveableCube`))
  (bind _moveablecube_4 (`self.MoveableCube`))
  (bind (_returnvalue_x _returnvalue_y _returnvalue_z) (`KismetMathLibrary.BreakVector` (`SceneComponent.K2_GetComponentLocation` _moveablecube_2)))
  (bind (_returnvalue_x_2 _returnvalue_y_2 _returnvalue_z_2) (`KismetMathLibrary.BreakVector` (`SceneComponent.K2_GetComponentLocation` _moveablecube_3)))
  ;[1 0.2543 0.6067] OverlapEvents
  (`|ExecutionSequence`
    (:`then_0`
      (bind _outhit (`KismetSystemLibrary.LineTraceSingle` :`Start` (`SceneComponent.K2_GetComponentLocation` _moveablecube_2) :`End` (`KismetMathLibrary.MakeVector` _returnvalue_x _returnvalue_y (+ _returnvalue_z 0.0)) :`TraceChannel` "TraceTypeQuery1" :`DrawDebugType` (`self.Draw Debug Type`)))
      (set `self.Out Hit Impact Point` (`.ImpactPoint` (`GameplayStatics.BreakHitResult` _outhit)))
      (set `self.Out Hit Hit Actor` (`.HitActor` (`GameplayStatics.BreakHitResult` _outhit)))
      (`/Engine/EditorBlueprintResources/StandardMacros.IsValid` (`.HitComponent` (`GameplayStatics.BreakHitResult` _outhit))
        (:`Is Not Valid`
          (set `self.MoveDirectionInt` 1))))
    (:`then_1`
      (bind _outhit_2 (`KismetSystemLibrary.LineTraceSingle` :`Start` (`SceneComponent.K2_GetComponentLocation` _moveablecube_3) :`End` (`KismetMathLibrary.MakeVector` _returnvalue_x_2 _returnvalue_y_2 (- _returnvalue_z_2 (`self.TracDistance`))) :`TraceChannel` "TraceTypeQuery1" :`DrawDebugType` (`self.Draw Debug Type`)))
      (`/Engine/EditorBlueprintResources/StandardMacros.IsValid` (`.HitComponent` (`GameplayStatics.BreakHitResult` _outhit_2))
        (:`Is Not Valid`
          (set `self.MoveDirectionInt` 2))))
    (:`then_2`
      (bind _outhit_3 (`KismetSystemLibrary.LineTraceSingle` :`Start` (`SceneComponent.K2_GetComponentLocation` _moveablecube_4) :`End` (* (* (`SceneComponent.GetForwardVector` _moveablecube_4) (`self.TracDistance`)) -1.0) :`TraceChannel` "TraceTypeQuery1" :`DrawDebugType` (`self.Draw Debug Type`)))
      (`/Engine/EditorBlueprintResources/StandardMacros.IsValid` (`.HitComponent` (`GameplayStatics.BreakHitResult` _outhit_3))
        (:`Is Not Valid`
          (set `self.MoveDirectionInt` 3))))
    (:`then_3`
      (bind _outhit_4 (`KismetSystemLibrary.LineTraceSingle` :`Start` (`SceneComponent.K2_GetComponentLocation` _moveablecube) :`End` (* (`SceneComponent.GetForwardVector` _moveablecube) (`self.TracDistance`)) :`TraceChannel` "TraceTypeQuery1" :`DrawDebugType` (`self.Draw Debug Type`)))
      (`/Engine/EditorBlueprintResources/StandardMacros.IsValid` (`.HitComponent` (`GameplayStatics.BreakHitResult` _outhit_4))
        (:`Is Not Valid`
          (set `self.MoveDirectionInt` 4))))
    (:`then_4`
      (`self.DirectionLogic`))))

(fn `GetDisplayText`
  (returns (DisplayText :type String))
  (return ""))

(fn `UserConstructionScript`)