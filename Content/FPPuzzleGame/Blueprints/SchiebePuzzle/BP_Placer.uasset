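; Placer actor that builds a 3x3 sliding-puzzle board from cubes one second after BeginPlay.
; It spawns ClassToSpawn at nine placeholder components, destroys each placeholder and collects the cubes in ListOfCubes.
; The SolveCubeIndex cube turns emissive red as the win cube, and the DeleteCubeIndex cube is destroyed, leaving a gap.
; ParseActor later attaches cubes to a supplied actor through nested validity checks, stopping at the first invalid cube.
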(event `SetMaterialWinCube`
  (bind _output (`|GetArrayItem` (`self.ListOfCubes`) (`self.SolveCubeIndex`)))
  ;[1 1 1] SetWinConCube
  (`/Engine/EditorBlueprintResources/StandardMacros.IsValid` _output
    (:`Is Valid`
      (`PrimitiveComponent.SetMaterial` (`self.GetComponentByClass` _output "/Script/Engine.StaticMeshComponent") 0 "/Game/FPPuzzleGame/Materials/General/M_EmissiveWallsRed.M_EmissiveWallsRed"))))

(event `AddToArray`
  (params (NewItem :type "Actor Object Reference (by ref)"))
  ;[1 1 1] MakeArrayOfCubes
  (`KismetArrayLibrary.Array_AddUnique` (`self.ListOfCubes`) NewItem))

(event `DestroyOneCube`
  (bind _output (`|GetArrayItem` (`self.ListOfCubes`) (`self.DeleteCubeIndex`)))
  ;[1 1 1] DestroyCube
  (`/Engine/EditorBlueprintResources/StandardMacros.IsValid` _output
    (:`Is Valid`
      (`self.K2_DestroyActor` _output))))

(event `ClearArray`
  (`KismetArrayLibrary.Array_Clear` (`self.ListOfCubes`)))

(event `self.ReceiveBeginPlay`
  (`KismetSystemLibrary.Delay` 1.0)
  (`self.SetActors`))

(event `SetActors`
  (bind _bottommid (`self.BottomMid`))
  (bind _midright (`self.MidRight`))
  (bind _mid (`self.Mid`))
  (bind _bottomleft (`self.BottomLeft`))
  (bind _topleft (`self.TopLeft`))
  (bind _topright (`self.TopRight`))
  (bind _topmid (`self.TopMid`))
  (bind _bottomright (`self.BottomRight`))
  (bind _midleft (`self.MidLeft`))
  ;[1 1 1] PopulateMiniGame
  (`|ExecutionSequence`
    (:`then_0`
      (bind _returnvalue (`|SpawnActorFromClass` (`self.ClassToSpawn`) (`SceneComponent.K2_GetComponentToWorld` _topleft) "Undefined" "OverrideRootScale" self null))
      (`ActorComponent.K2_DestroyComponent` _topleft)
      (`self.AddToArray` _returnvalue))
    (:`then_1`
      (bind _returnvalue_2 (`|SpawnActorFromClass` (`self.ClassToSpawn`) (`SceneComponent.K2_GetComponentToWorld` _topmid) "Undefined" "OverrideRootScale" self null))
      (`ActorComponent.K2_DestroyComponent` _topmid)
      (`self.AddToArray` _returnvalue_2))
    (:`then_2`
      (bind _returnvalue_3 (`|SpawnActorFromClass` (`self.ClassToSpawn`) (`SceneComponent.K2_GetComponentToWorld` _topright) "Undefined" "OverrideRootScale" self null))
      (`ActorComponent.K2_DestroyComponent` _topright)
      (`self.AddToArray` _returnvalue_3))
    (:`then_3`
      (bind _returnvalue_4 (`|SpawnActorFromClass` (`self.ClassToSpawn`) (`SceneComponent.K2_GetComponentToWorld` _midleft) "Undefined" "OverrideRootScale" self null))
      (`ActorComponent.K2_DestroyComponent` _midleft)
      (`self.AddToArray` _returnvalue_4))
    (:`then_4`
      (bind _returnvalue_5 (`|SpawnActorFromClass` (`self.ClassToSpawn`) (`SceneComponent.K2_GetComponentToWorld` _mid) "Undefined" "OverrideRootScale" self null))
      (`ActorComponent.K2_DestroyComponent` _mid)
      (`self.AddToArray` _returnvalue_5))
    (:`then_5`
      (bind _returnvalue_6 (`|SpawnActorFromClass` (`self.ClassToSpawn`) (`SceneComponent.K2_GetComponentToWorld` _midright) "Undefined" "OverrideRootScale" self null))
      (`ActorComponent.K2_DestroyComponent` _midright)
      (`self.AddToArray` _returnvalue_6))
    (:`then_6`
      (bind _returnvalue_7 (`|SpawnActorFromClass` (`self.ClassToSpawn`) (`SceneComponent.K2_GetComponentToWorld` _bottommid) "Undefined" "OverrideRootScale" self null))
      (`ActorComponent.K2_DestroyComponent` _bottommid)
      (`self.AddToArray` _returnvalue_7))
    (:`then_7`
      (bind _returnvalue_8 (`|SpawnActorFromClass` (`self.ClassToSpawn`) (`SceneComponent.K2_GetComponentToWorld` _bottomleft) "Undefined" "OverrideRootScale" self null))
      (`ActorComponent.K2_DestroyComponent` _bottomleft)
      (`self.AddToArray` _returnvalue_8))
    (:`then_8`
      (bind _returnvalue_9 (`|SpawnActorFromClass` (`self.ClassToSpawn`) (`SceneComponent.K2_GetComponentToWorld` _bottomright) "Undefined" "OverrideRootScale" self null))
      (`ActorComponent.K2_DestroyComponent` _bottomright)
      (`self.AddToArray` _returnvalue_9))
    (:`then_9`
      (`self.SetMaterialWinCube`)
      (`self.DestroyOneCube`))))

(event `SetNewParent`
  (bind _location_rule (`self.Location Rule`))
  (bind _location_rule_2 (`self.Location Rule`))
  (bind _location_rule_3 (`self.Location Rule`))
  (bind _location_rule_4 (`self.Location Rule`))
  (bind _location_rule_5 (`self.Location Rule`))
  (bind _location_rule_6 (`self.Location Rule`))
  (bind _location_rule_7 (`self.Location Rule`))
  (bind _location_rule_8 (`self.Location Rule`))
  (bind _location_rule_9 (`self.Location Rule`))
  (`/Engine/EditorBlueprintResources/StandardMacros.IsValid` (stale `SetActors` _returnvalue_9)
    (:`Is Valid`
      (`self.K2_AttachToActor` (stale `SetActors` _returnvalue_9) (`self.NewParentForSingleCubes`) "None" _location_rule _location_rule _location_rule false)
      (`/Engine/EditorBlueprintResources/StandardMacros.IsValid` (stale `SetActors` _returnvalue_8)
        (:`Is Valid`
          (`self.K2_AttachToActor` (stale `SetActors` _returnvalue_8) (`self.NewParentForSingleCubes`) "None" _location_rule_2 _location_rule_2 _location_rule_2 false)
          (`/Engine/EditorBlueprintResources/StandardMacros.IsValid` (stale `SetActors` _returnvalue_7)
            (:`Is Valid`
              (`self.K2_AttachToActor` (stale `SetActors` _returnvalue_7) (`self.NewParentForSingleCubes`) "None" _location_rule_3 _location_rule_3 _location_rule_3 false)
              (`/Engine/EditorBlueprintResources/StandardMacros.IsValid` (stale `SetActors` _returnvalue_6)
                (:`Is Valid`
                  (`self.K2_AttachToActor` (stale `SetActors` _returnvalue_6) (`self.NewParentForSingleCubes`) "None" _location_rule_4 _location_rule_4 _location_rule_4 false)
                  (`/Engine/EditorBlueprintResources/StandardMacros.IsValid` (stale `SetActors` _returnvalue_5)
                    (:`Is Valid`
                      (`self.K2_AttachToActor` (stale `SetActors` _returnvalue_5) (`self.NewParentForSingleCubes`) "None" _location_rule_5 _location_rule_5 _location_rule_5 false)
                      (`/Engine/EditorBlueprintResources/StandardMacros.IsValid` (stale `SetActors` _returnvalue_4)
                        (:`Is Valid`
                          (`self.K2_AttachToActor` (stale `SetActors` _returnvalue_4) (`self.NewParentForSingleCubes`) "None" _location_rule_6 _location_rule_6 _location_rule_6 false)
                          (`/Engine/EditorBlueprintResources/StandardMacros.IsValid` (stale `SetActors` _returnvalue_3)
                            (:`Is Valid`
                              (`self.K2_AttachToActor` (stale `SetActors` _returnvalue_3) (`self.NewParentForSingleCubes`) "None" _location_rule_7 _location_rule_7 _location_rule_7 false)
                              (`/Engine/EditorBlueprintResources/StandardMacros.IsValid` (stale `SetActors` _returnvalue_2)
                                (:`Is Valid`
                                  (`self.K2_AttachToActor` (stale `SetActors` _returnvalue_2) (`self.NewParentForSingleCubes`) "None" _location_rule_8 _location_rule_8 _location_rule_8 false)
                                  (`/Engine/EditorBlueprintResources/StandardMacros.IsValid` (stale `SetActors` _returnvalue)
                                    (:`Is Valid`
                                      (`self.K2_AttachToActor` (stale `SetActors` _returnvalue) (`self.NewParentForSingleCubes`) "None" _location_rule_9 _location_rule_9 _location_rule_9 false))))))))))))))))))))

(event `/Game/FPPuzzleGame/Blueprints/Interfaces/BPI_Trigger.ParseActor`
  (params (Actor :type "Actor Object Reference"))
  (set `self.NewParentForSingleCubes` Actor)
  (`KismetSystemLibrary.PrintString` "Hello")
  (`KismetSystemLibrary.Delay` 0.2)
  (`self.SetNewParent`))

(fn `UserConstructionScript`)