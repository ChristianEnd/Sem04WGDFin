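; Interactable controller in the sliding puzzle (SchiebePuzzle) whose Turnable component rotates when used.
; Focus toggles custom depth rendering on Turnable, presumably for highlighting.
; Interact plays a slowed timeline that lerps toward a target built from the stored world pitch plus 90 degrees, applied as relative rotation.
; A DoOnce blocks repeat input until the animation finishes, when the stored world rotation is refreshed.
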(event `/Game/FPPuzzleGame/Blueprints/Interfaces/BPI_Interact.SetFocus`
  (params (IsFocused :type Boolean))
  (`PrimitiveComponent.SetRenderCustomDepth` (`self.Turnable`) IsFocused))

(event `self.ReceiveBeginPlay`
  (`TimelineComponent.SetPlayRate` (`self.ANIM`) 0.25)
  (set `self.WorldRotPlacer` (`SceneComponent.K2_GetComponentRotation` (`self.Turnable`))))

(event `/Game/FPPuzzleGame/Blueprints/Interfaces/BPI_Interact.Interact`
  (bind (_worldrotplacer_roll _worldrotplacer_pitch) (`KismetMathLibrary.BreakRotator` (`self.WorldRotPlacer`)))
  (`/Engine/EditorBlueprintResources/StandardMacros.DoOnce` false :!label _label
    (:`Completed`
      (set `self.NewRot` (`KismetMathLibrary.MakeRotator` 0.0 (+ _worldrotplacer_pitch 90.0)))
      (bind (_direction _alpha) (`Timeline|ANIM` :!via `PlayFromStart`)
        (:`Update`
          (`SceneComponent.K2_SetRelativeRotation` (`self.Turnable`) (`KismetMathLibrary.RLerp` (`self.WorldRotPlacer`) (`self.NewRot`) _alpha) false false))
        (:`Finished`
          (`self.UnlockRotation`)
          (set `self.WorldRotPlacer` (`SceneComponent.K2_GetComponentRotation` (`self.Turnable`))))))))

(event `UnlockRotation`
  (goto _label :!via `Reset`))

(fn `GetDisplayText`
  (returns (DisplayText :type String))
  (return ""))

(fn `UserConstructionScript`)