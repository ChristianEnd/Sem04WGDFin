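; Puzzle placer actor for the SchiebePuzzle (sliding puzzle) that spawns four attached 3x3 cube grids, each with one cube removed and one given a colored win material.
; The root starts at a random multiple of 90° pitch, and Trigger turns it another step.
; ReverseTrigger line-traces along +Y from each colored cube, comparing materials on BPI_Puzzle hits, and sends TriggerMessage to WinActors when all four match.
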(event `AddToArray`
  (params (NewItem :type "Actor Object Reference (by ref)"))
  ;[1 1 1] MakeArrayOfCubes
  (`KismetArrayLibrary.Array_AddUnique` (`self.ListOfCubes`) NewItem))

(event `DestroyOneCube`
  (bind _output (`|GetArrayItem` (`self.ListOfCubes`) (`self.DeleteCubeIndex`)))
  ;[1 1 1] DestroyCube
  (`/Engine/EditorBlueprintResources/StandardMacros.IsValid` _output
    (:`Is Valid`
      (`self.K2_DestroyActor` _output))))

(event `SetMaterialWinCube`
  (bind _output (`|GetArrayItem` (`self.ListOfCubes`) (`self.SolveCubeIndex`)))
  ;[1 1 1] SetWinConCube
  (set `self.WinConCube00` _output)
  (`/Engine/EditorBlueprintResources/StandardMacros.IsValid` _output
    (:`Is Valid`
      (`PrimitiveComponent.SetMaterial` (`self.GetComponentByClass` _output "/Script/Engine.StaticMeshComponent") 0 "/Game/FPPuzzleGame/Materials/General/M_EmissiveWallsRed.M_EmissiveWallsRed"))))

(event `ClearArray`
  ;[1 1 1] MakeArrayOfCubes
  (`KismetArrayLibrary.Array_Clear` (`self.ListOfCubes`)))

(event `DestroyOneCube1`
  (bind _output (`|GetArrayItem` (`self.ListOfCubes_0`) (`self.DeleteCubeIndex`)))
  ;[1 1 1] DestroyCube
  (`/Engine/EditorBlueprintResources/StandardMacros.IsValid` _output
    (:`Is Valid`
      (`self.K2_DestroyActor` _output))))

(event `AddToArray1`
  (params (NewItem :type "Actor Object Reference (by ref)"))
  ;[1 1 1] MakeArrayOfCubes
  (`KismetArrayLibrary.Array_AddUnique` (`self.ListOfCubes_0`) NewItem))

(event `SetMaterialWinCube1`
  (bind _output (`|GetArrayItem` (`self.ListOfCubes_0`) (`self.SolveCubeIndex`)))
  ;[1 1 1] SetWinConCube
  (set `self.WinConCube01` _output)
  (`/Engine/EditorBlueprintResources/StandardMacros.IsValid` _output
    (:`Is Valid`
      (`PrimitiveComponent.SetMaterial` (`self.GetComponentByClass` _output "/Script/Engine.StaticMeshComponent") 0 "/Game/FPPuzzleGame/Materials/General/M_MI_E_Purple.M_MI_E_Purple"))))

(event `DestroyOneCube2`
  (bind _output (`|GetArrayItem` (`self.ListOfCubes_1`) (`self.DeleteCubeIndex`)))
  ;[1 1 1] DestroyCube
  (`/Engine/EditorBlueprintResources/StandardMacros.IsValid` _output
    (:`Is Valid`
      (`self.K2_DestroyActor` _output))))

(event `ClearArray1`
  ;[1 1 1] MakeArrayOfCubes
  (`KismetArrayLibrary.Array_Clear` (`self.ListOfCubes_0`)))

(event `SetMaterialWinCube2`
  (bind _output (`|GetArrayItem` (`self.ListOfCubes_1`) (`self.SolveCubeIndex`)))
  ;[1 1 1] SetWinConCube
  (set `self.WinConCube02` _output)
  (`/Engine/EditorBlueprintResources/StandardMacros.IsValid` _output
    (:`Is Valid`
      (`PrimitiveComponent.SetMaterial` (`self.GetComponentByClass` _output "/Script/Engine.StaticMeshComponent") 0 "/Game/FPPuzzleGame/Materials/General/M_MI_E_Green.M_MI_E_Green"))))

(event `AddToArray2`
  (params (NewItem :type "Actor Object Reference (by ref)"))
  ;[1 1 1] MakeArrayOfCubes
  (`KismetArrayLibrary.Array_AddUnique` (`self.ListOfCubes_1`) NewItem))

(event `DestroyOneCube3`
  (bind _output (`|GetArrayItem` (`self.ListOfCubes_2`) (`self.DeleteCubeIndex`)))
  ;[1 1 1] DestroyCube
  (`/Engine/EditorBlueprintResources/StandardMacros.IsValid` _output
    (:`Is Valid`
      (`self.K2_DestroyActor` _output))))

(event `ClearArray2`
  ;[1 1 1] MakeArrayOfCubes
  (`KismetArrayLibrary.Array_Clear` (`self.ListOfCubes_1`)))

(event `SetMaterialWinCube3`
  (bind _output (`|GetArrayItem` (`self.ListOfCubes_2`) (`self.SolveCubeIndex`)))
  ;[1 1 1] SetWinConCube
  (set `self.WinConCube03` _output)
  (`/Engine/EditorBlueprintResources/StandardMacros.IsValid` _output
    (:`Is Valid`
      (`PrimitiveComponent.SetMaterial` (`self.GetComponentByClass` _output "/Script/Engine.StaticMeshComponent") 0 "/Game/FPPuzzleGame/Materials/General/M_MI_E_Yellow.M_MI_E_Yellow"))))

(event `AddToArray3`
  (params (NewItem :type "Actor Object Reference (by ref)"))
  ;[1 1 1] MakeArrayOfCubes
  (`KismetArrayLibrary.Array_AddUnique` (`self.ListOfCubes_2`) NewItem))

(event `ClearArray3`
  ;[1 1 1] MakeArrayOfCubes
  (`KismetArrayLibrary.Array_Clear` (`self.ListOfCubes_2`)))

(event `self.ReceiveBeginPlay`
  ;[1 1 1] Start
  (`KismetSystemLibrary.Delay` 1.0)
  (`self.SetActors`)
  (`self.SetActors1`)
  (`self.SetActors2`)
  (`self.SetActors3`)
  (`self.RandomStartRotation`))

(event `/Game/FPPuzzleGame/Blueprints/Interfaces/BPI_Trigger.Trigger`
  ;[1 1 1] Rotate
  (`SceneComponent.K2_AddWorldRotation` (`self.DefaultSceneRoot`) (`KismetMathLibrary.MakeRotator` 0.0 90.0) false false))

(event `RandomStartRotation`
  ;[1 1 1] StartRandomLoop
  (set `self.Fin` (`KismetMathLibrary.RandomIntegerInRange` 2 12))
  (if (not (== (`self.Counter`) (`self.Fin`))) :!label _label
    (`SceneComponent.K2_AddWorldRotation` (`self.DefaultSceneRoot`) (`KismetMathLibrary.MakeRotator` 0.0 90.0) false false)
    (`/Engine/EditorBlueprintResources/StandardMacros.IncrementInt` (`self.Counter`)
      (:`  `
        (goto _label)))))

(event `SetActors`
  (bind _location_rule (`self.Location Rule`))
  (bind _location_rule_2 (`self.Location Rule`))
  (bind _location_rule_3 (`self.Location Rule`))
  (bind _location_rule_4 (`self.Location Rule`))
  (bind _location_rule_5 (`self.Location Rule`))
  (bind _location_rule_6 (`self.Location Rule`))
  (bind _location_rule_7 (`self.Location Rule`))
  (bind _location_rule_8 (`self.Location Rule`))
  (bind _location_rule_9 (`self.Location Rule`))
  (bind _bottommid (`self.BottomMid`))
  (bind _midright (`self.MidRight`))
  (bind _mid (`self.Mid`))
  (bind _bottomleft (`self.BottomLeft`))
  (bind _topleft (`self.TopLeft`))
  (bind _topright (`self.TopRight`))
  (bind _topmid (`self.TopMid`))
  (bind _bottomright (`self.BottomRight`))
  (bind _midleft (`self.MidLeft`))
  ;[1 1 1] PopulateMiniGame
  (`|ExecutionSequence`
    (:`then_0`
      (bind _returnvalue (`|SpawnActorFromClass` (`self.ClassToSpawn`) (`SceneComponent.K2_GetComponentToWorld` _topleft) "Undefined" "OverrideRootScale" self null))
      (`ActorComponent.K2_DestroyComponent` _topleft)
      (`self.AddToArray` _returnvalue))
    (:`then_1`
      (bind _returnvalue_2 (`|SpawnActorFromClass` (`self.ClassToSpawn`) (`SceneComponent.K2_GetComponentToWorld` _topmid) "Undefined" "OverrideRootScale" self null))
      (`ActorComponent.K2_DestroyComponent` _topmid)
      (`self.AddToArray` _returnvalue_2))
    (:`then_2`
      (bind _returnvalue_3 (`|SpawnActorFromClass` (`self.ClassToSpawn`) (`SceneComponent.K2_GetComponentToWorld` _topright) "Undefined" "OverrideRootScale" self null))
      (`ActorComponent.K2_DestroyComponent` _topright)
      (`self.AddToArray` _returnvalue_3))
    (:`then_3`
      (bind _returnvalue_4 (`|SpawnActorFromClass` (`self.ClassToSpawn`) (`SceneComponent.K2_GetComponentToWorld` _midleft) "Undefined" "OverrideRootScale" self null))
      (`ActorComponent.K2_DestroyComponent` _midleft)
      (`self.AddToArray` _returnvalue_4))
    (:`then_4`
      (bind _returnvalue_5 (`|SpawnActorFromClass` (`self.ClassToSpawn`) (`SceneComponent.K2_GetComponentToWorld` _mid) "Undefined" "OverrideRootScale" self null))
      (`ActorComponent.K2_DestroyComponent` _mid)
      (`self.AddToArray` _returnvalue_5))
    (:`then_5`
      (bind _returnvalue_6 (`|SpawnActorFromClass` (`self.ClassToSpawn`) (`SceneComponent.K2_GetComponentToWorld` _midright) "Undefined" "OverrideRootScale" self null))
      (`ActorComponent.K2_DestroyComponent` _midright)
      (`self.AddToArray` _returnvalue_6))
    (:`then_6`
      (bind _returnvalue_7 (`|SpawnActorFromClass` (`self.ClassToSpawn`) (`SceneComponent.K2_GetComponentToWorld` _bottommid) "Undefined" "OverrideRootScale" self null))
      (`ActorComponent.K2_DestroyComponent` _bottommid)
      (`self.AddToArray` _returnvalue_7))
    (:`then_7`
      (bind _returnvalue_8 (`|SpawnActorFromClass` (`self.ClassToSpawn`) (`SceneComponent.K2_GetComponentToWorld` _bottomleft) "Undefined" "OverrideRootScale" self null))
      (`ActorComponent.K2_DestroyComponent` _bottomleft)
      (`self.AddToArray` _returnvalue_8))
    (:`then_8`
      (bind _returnvalue_9 (`|SpawnActorFromClass` (`self.ClassToSpawn`) (`SceneComponent.K2_GetComponentToWorld` _bottomright) "Undefined" "OverrideRootScale" self null))
      (`ActorComponent.K2_DestroyComponent` _bottomright)
      (`self.AddToArray` _returnvalue_9)
      (`/Engine/EditorBlueprintResources/StandardMacros.IsValid` _returnvalue_9
        (:`Is Valid`
          (`self.K2_AttachToActor` _returnvalue_9 self "None" _location_rule_9 _location_rule_9 _location_rule_9 false)
          (`/Engine/EditorBlueprintResources/StandardMacros.IsValid` _returnvalue_8
            (:`Is Valid`
              (`self.K2_AttachToActor` _returnvalue_8 self "None" _location_rule _location_rule _location_rule false)
              (`/Engine/EditorBlueprintResources/StandardMacros.IsValid` _returnvalue_7
                (:`Is Valid`
                  (`self.K2_AttachToActor` _returnvalue_7 self "None" _location_rule_2 _location_rule_2 _location_rule_2 false)
                  (`/Engine/EditorBlueprintResources/StandardMacros.IsValid` _returnvalue_6
                    (:`Is Valid`
                      (`self.K2_AttachToActor` _returnvalue_6 self "None" _location_rule_3 _location_rule_3 _location_rule_3 false)
                      (`/Engine/EditorBlueprintResources/StandardMacros.IsValid` _returnvalue_5
                        (:`Is Valid`
                          (`self.K2_AttachToActor` _returnvalue_5 self "None" _location_rule_4 _location_rule_4 _location_rule_4 false)
                          (`/Engine/EditorBlueprintResources/StandardMacros.IsValid` _returnvalue_4
                            (:`Is Valid`
                              (`self.K2_AttachToActor` _returnvalue_4 self "None" _location_rule_5 _location_rule_5 _location_rule_5 false)
                              (`/Engine/EditorBlueprintResources/StandardMacros.IsValid` _returnvalue_3
                                (:`Is Valid`
                                  (`self.K2_AttachToActor` _returnvalue_3 self "None" _location_rule_6 _location_rule_6 _location_rule_6 false)
                                  (`/Engine/EditorBlueprintResources/StandardMacros.IsValid` _returnvalue_2
                                    (:`Is Valid`
                                      (`self.K2_AttachToActor` _returnvalue_2 self "None" _location_rule_7 _location_rule_7 _location_rule_7 false)
                                      (`/Engine/EditorBlueprintResources/StandardMacros.IsValid` _returnvalue
                                        (:`Is Valid`
                                          (`self.K2_AttachToActor` _returnvalue self "None" _location_rule_8 _location_rule_8 _location_rule_8 false))))))))))))))))))))
    (:`then_9`
      (`self.SetMaterialWinCube`)
      (`self.DestroyOneCube`))))

(event `SetActors1`
  (bind _location_rule (`self.Location Rule`))
  ;[1 1 1] PopulateMiniGame
  (for _array_element (`|MakeArray` (`self.StaticMesh20`) (`self.StaticMesh19`) (`self.StaticMesh18`) (`self.StaticMesh17`) (`self.StaticMesh22`) (`self.StaticMesh16`) (`self.StaticMesh21`) (`self.BottomRight3`) (`self.StaticMesh23`))
    (bind _returnvalue (`|SpawnActorFromClass` (`self.ClassToSpawn`) (`SceneComponent.K2_GetComponentToWorld` _array_element) "Undefined" "OverrideRootScale" self null))
    (`self.AddToArray1` _returnvalue)
    (`self.K2_AttachToActor` _returnvalue self "None" _location_rule _location_rule _location_rule false))
  (`self.DestroyOneCube1`)
  (`self.SetMaterialWinCube1`))

(event `SetActors2`
  (bind _location_rule (`self.Location Rule`))
  ;[1 1 1] PopulateMiniGame
  (for _array_element (`|MakeArray` (`self.StaticMesh2`) (`self.StaticMesh4`) (`self.StaticMesh3`) (`self.StaticMesh`) (`self.StaticMesh5`) (`self.StaticMesh1`) (`self.StaticMesh6`) (`self.BottomRight1`) (`self.StaticMesh7`))
    (bind _returnvalue (`|SpawnActorFromClass` (`self.ClassToSpawn`) (`SceneComponent.K2_GetComponentToWorld` _array_element) "Undefined" "OverrideRootScale" self null))
    (`self.AddToArray2` _returnvalue)
    (`self.K2_AttachToActor` _returnvalue self "None" _location_rule _location_rule _location_rule false))
  (`self.DestroyOneCube2`)
  (`self.SetMaterialWinCube2`))

(event `SetActors3`
  (bind _location_rule (`self.Location Rule`))
  ;[1 1 1] PopulateMiniGame
  (for _array_element (`|MakeArray` (`self.StaticMesh10`) (`self.StaticMesh13`) (`self.StaticMesh12`) (`self.StaticMesh11`) (`self.StaticMesh8`) (`self.StaticMesh9`) (`self.StaticMesh15`) (`self.BottomRight2`) (`self.StaticMesh14`))
    (bind _returnvalue (`|SpawnActorFromClass` (`self.ClassToSpawn`) (`SceneComponent.K2_GetComponentToWorld` _array_element) "Undefined" "OverrideRootScale" self null))
    (`self.AddToArray3` _returnvalue)
    (`self.K2_AttachToActor` _returnvalue self "None" _location_rule _location_rule _location_rule false))
  (`self.DestroyOneCube3`)
  (`self.SetMaterialWinCube3`))

(event `WinEvent`
  (`KismetSystemLibrary.PrintString` "WinEvent")
  (for _array_element (`self.WinActors`)
    (message `/Game/FPPuzzleGame/Blueprints/Interfaces/BPI_Trigger.Trigger` _array_element)))

(event `/Game/FPPuzzleGame/Blueprints/Interfaces/BPI_Trigger.ReverseTrigger`
  (`self.CheckWin`))

(event `CheckWin`
  (bind _winconcube01 (`self.WinConCube01`))
  (bind _winconcube02 (`self.WinConCube02`))
  (bind _winconcube03 (`self.WinConCube03`))
  (bind _winconcube00 (`self.WinConCube00`))
  (bind (_returnvalue_x _returnvalue_y _returnvalue_z) (`KismetMathLibrary.BreakVector` (`self.K2_GetActorLocation` _winconcube01)))
  (bind (_returnvalue_x_2 _returnvalue_y_2 _returnvalue_z_2) (`KismetMathLibrary.BreakVector` (`self.K2_GetActorLocation` _winconcube01)))
  (bind (_returnvalue_x_3 _returnvalue_y_3 _returnvalue_z_3) (`KismetMathLibrary.BreakVector` (`self.K2_GetActorLocation` _winconcube00)))
  (bind (_returnvalue_x_4 _returnvalue_y_4 _returnvalue_z_4) (`KismetMathLibrary.BreakVector` (`self.K2_GetActorLocation` _winconcube00)))
  (bind (_returnvalue_x_5 _returnvalue_y_5 _returnvalue_z_5) (`KismetMathLibrary.BreakVector` (`self.K2_GetActorLocation` _winconcube02)))
  (bind (_returnvalue_x_6 _returnvalue_y_6 _returnvalue_z_6) (`KismetMathLibrary.BreakVector` (`self.K2_GetActorLocation` _winconcube02)))
  (bind (_returnvalue_x_7 _returnvalue_y_7 _returnvalue_z_7) (`KismetMathLibrary.BreakVector` (`self.K2_GetActorLocation` _winconcube03)))
  (bind (_returnvalue_x_8 _returnvalue_y_8 _returnvalue_z_8) (`KismetMathLibrary.BreakVector` (`self.K2_GetActorLocation` _winconcube03)))
  (`|ExecutionSequence`
    (:`then_0`
      (bind _outhit (`KismetSystemLibrary.LineTraceSingle` (`KismetMathLibrary.MakeVector` _returnvalue_x_3 (+ _returnvalue_y_3 100.0) _returnvalue_z_3) (`KismetMathLibrary.MakeVector` _returnvalue_x_4 (+ _returnvalue_y_4 1000.0) _returnvalue_z_4) "TraceTypeQuery1" false (`self.ListOfCubes`) "ForDuration" true (struct :`R` 1.0 :`A` 1.0) (struct :`G` 1.0 :`A` 1.0) 15.0))
      (if (`KismetSystemLibrary.DoesImplementInterface` (`.HitActor` (`GameplayStatics.BreakHitResult` _outhit)) "/Game/FPPuzzleGame/Blueprints/Interfaces/BPI_Puzzle.BPI_Puzzle_C")
        (if (== (`PrimitiveComponent.GetMaterial` (`.HitComponent` (`GameplayStatics.BreakHitResult` _outhit)) 0) (`PrimitiveComponent.GetMaterial` (`self.GetComponentByClass` _winconcube00 "/Script/Engine.StaticMeshComponent") 0))
          (set `self.Bool00` true)
          (else
            (set `self.Bool00` false)))))
    (:`then_1`
      (bind _outhit_2 (`KismetSystemLibrary.LineTraceSingle` (`KismetMathLibrary.MakeVector` _returnvalue_x_5 (+ _returnvalue_y_5 100.0) _returnvalue_z_5) (`KismetMathLibrary.MakeVector` _returnvalue_x_6 (+ _returnvalue_y_6 1000.0) _returnvalue_z_6) "TraceTypeQuery1" false (`self.ListOfCubes_0`) "ForDuration" true (struct :`R` 1.0 :`A` 1.0) (struct :`G` 1.0 :`A` 1.0) 15.0))
      (if (`KismetSystemLibrary.DoesImplementInterface` (`.HitActor` (`GameplayStatics.BreakHitResult` _outhit_2)) "/Game/FPPuzzleGame/Blueprints/Interfaces/BPI_Puzzle.BPI_Puzzle_C")
        (if (== (`PrimitiveComponent.GetMaterial` (`.HitComponent` (`GameplayStatics.BreakHitResult` _outhit_2)) 0) (`PrimitiveComponent.GetMaterial` (`self.GetComponentByClass` _winconcube02 "/Script/Engine.StaticMeshComponent") 0))
          (set `self.Bool00_0` true)
          (else
            (set `self.Bool00_0` false)))))
    (:`then_2`
      (bind _outhit_3 (`KismetSystemLibrary.LineTraceSingle` (`KismetMathLibrary.MakeVector` _returnvalue_x_7 (+ _returnvalue_y_7 100.0) _returnvalue_z_7) (`KismetMathLibrary.MakeVector` _returnvalue_x_8 (+ _returnvalue_y_8 1000.0) _returnvalue_z_8) "TraceTypeQuery1" false (`self.ListOfCubes_1`) "ForDuration" true (struct :`R` 1.0 :`A` 1.0) (struct :`G` 1.0 :`A` 1.0) 15.0))
      (if (`KismetSystemLibrary.DoesImplementInterface` (`.HitActor` (`GameplayStatics.BreakHitResult` _outhit_3)) "/Game/FPPuzzleGame/Blueprints/Interfaces/BPI_Puzzle.BPI_Puzzle_C")
        (if (== (`PrimitiveComponent.GetMaterial` (`.HitComponent` (`GameplayStatics.BreakHitResult` _outhit_3)) 0) (`PrimitiveComponent.GetMaterial` (`self.GetComponentByClass` _winconcube03 "/Script/Engine.StaticMeshComponent") 0))
          (set `self.Bool00_1` true)
          (else
            (set `self.Bool00_1` false)))))
    (:`then_3`
      (bind _outhit_4 (`KismetSystemLibrary.LineTraceSingle` :`Start` (`KismetMathLibrary.MakeVector` _returnvalue_x_2 (+ _returnvalue_y_2 100.0) _returnvalue_z_2) :`End` (`KismetMathLibrary.MakeVector` _returnvalue_x (+ _returnvalue_y 1000.0) _returnvalue_z) :`TraceChannel` "TraceTypeQuery1" :`DrawDebugType` "ForDuration" :`DrawTime` 15.0))
      (if (`KismetSystemLibrary.DoesImplementInterface` (`.HitActor` (`GameplayStatics.BreakHitResult` _outhit_4)) "/Game/FPPuzzleGame/Blueprints/Interfaces/BPI_Puzzle.BPI_Puzzle_C")
        (if (== (`PrimitiveComponent.GetMaterial` (`.HitComponent` (`GameplayStatics.BreakHitResult` _outhit_4)) 0) (`PrimitiveComponent.GetMaterial` (`self.GetComponentByClass` _winconcube01 "/Script/Engine.StaticMeshComponent") 0))
          (set `self.Bool00_2` true)
          (else
            (set `self.Bool00_2` false)))))
    (:`then_4`
      (if (and (`self.Bool00`) (`self.Bool00_0`) (`self.Bool00_1`) (`self.Bool00_2`))
        (`KismetSystemLibrary.PrintString` "AllTrue")
        (`self.WinEvent`)))))

(fn `GetDisplayText`
  (returns (DisplayText :type String))
  (return ""))

(fn `UserConstructionScript`)