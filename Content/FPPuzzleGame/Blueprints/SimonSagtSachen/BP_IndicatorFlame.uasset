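; BP_IndicatorFlame is a toggleable purple fire indicator with sound, apparently for the Simon Says puzzle.
; Burn spawns a Niagara fire system at the SystemLocation component, stores it as ActiveSystem and plays FMOD audio, guarded by a DoOnce against stacking flames.
; StopBurn destroys a valid ActiveSystem, re-arms the DoOnce through Reset and stops the audio.
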(event `Burn`
  (`/Engine/EditorBlueprintResources/StandardMacros.DoOnce` false :!label _label
    (:`Completed`
      (bind _returnvalue (`NiagaraFunctionLibrary.SpawnSystemAtLocation` "/Game/FPPuzzleGame/VFX/Fire/NS_Fire_Purple.NS_Fire_Purple" (`SceneComponent.K2_GetComponentLocation` (`self.SystemLocation`))))
      (set `self.ActiveSystem` _returnvalue)
      (`FMODAudioComponent.Play` (`self.FMODAudio`)))))

(event `Reset`
  (goto _label :!via `Reset`))

(event `StopBurn`
  (bind _activesystem (`self.ActiveSystem`))
  (`/Engine/EditorBlueprintResources/StandardMacros.IsValid` _activesystem
    (:`Is Valid`
      (`ActorComponent.K2_DestroyComponent` _activesystem)
      (`self.Reset`)
      (`FMODAudioComponent.Stop` (`self.FMODAudio`)))))

(fn `UserConstructionScript`)