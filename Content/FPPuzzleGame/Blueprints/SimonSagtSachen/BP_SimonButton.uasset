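; Interactable button for the Simon Says puzzle that reports its color value to the Simon module.
; Every press plays an FMOD sound and a timeline that slides the lower button mesh.
; Only an initialized button activates its linked buttons, triggers the module and starts the optional FireDis effect with that color.
; Focus highlighting through custom depth is likewise limited to initialized buttons.
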(event `/Game/FPPuzzleGame/Blueprints/Interfaces/BPI_Interact.Interact`
  (bind _switch_int_color (`self.Switch Int Color`))
  (bind _firedis (`self.FireDis`))
  (bind _otherbuttons (`self.OtherButtons`))
  ;[1 1 1] InteractionTowardsSimon
  (`self.ButtonAnim`)
  (if (`self.InitButton`)
    (if (not (`KismetArrayLibrary.Array_IsEmpty` _otherbuttons))
      (for _array_element _otherbuttons
        (`self.SetButtonActive` _array_element)))
    (`/Game/FPPuzzleGame/Blueprints/SimonSagtSachen/BP_SimonPuzzle.ValueTrigger` (`self.SimonModule`) _switch_int_color)
    (`/Engine/EditorBlueprintResources/StandardMacros.IsValid` _firedis
      (:`Is Valid`
        (`/Game/FPPuzzleGame/Blueprints/SimonSagtSachen/BP_SimonFlameDispenser.StartFire` _firedis _switch_int_color)))))

(event `/Game/FPPuzzleGame/Blueprints/Interfaces/BPI_Interact.SetFocus`
  (params (IsFocused :type Boolean))
  ;[1 1 1] SetFocus
  (if (`self.InitButton`)
    (`PrimitiveComponent.SetRenderCustomDepth` (`self.Button_low`) IsFocused)))

(event `SetButtonActive`
  (set `self.InitButton` true))

(event `ButtonAnim`
  (`FMODAudioComponent.Play` (`self.FMODAudio`))
  (bind (_direction _alpha) (`Timeline|Anim` :!via `PlayFromStart`)
    (:`Update`
      (`SceneComponent.K2_SetRelativeLocation` (`self.Button_low`) (`KismetMathLibrary.VLerp` (0.0 -2.0 0.0) (0.0 2.0 0.0) _alpha) false false))))

(fn `GetDisplayText`
  (returns (DisplayText :type String))
  (return ""))

(fn `UserConstructionScript`)