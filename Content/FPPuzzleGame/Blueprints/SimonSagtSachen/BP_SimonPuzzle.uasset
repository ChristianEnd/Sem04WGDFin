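; Simon Says puzzle Blueprint that plays a random sequence on fire displays for the player to repeat with four colour switches.
; ValueTrigger starts a round or checks each colour press against Playlist, while Start re-calls itself with a Delay to step through playback.
; A mistake resets to the first difficulty; a correct sequence advances it until the win condition notifies linked actors.
; Tick refreshes the progress indicator flames from Difficulty.
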(event `SetupDifficulty`
  ;[0 1 0.7656] SetupDifficulty
  (`KismetArrayLibrary.Array_Clear` (`self.Playlist`))
  (switch `int` (`self.Difficulty`)
    (:`1`
      (set `self.ToRemember` 3)
      (set `self.Speed` 2.0))
    (:`2`
      (set `self.ToRemember` 3)
      (set `self.Speed` 1.0))
    (:`3`
      (set `self.ToRemember` 3)
      (set `self.Speed` 1.0))))

(event `CreatePlaylist`
  ;[0.8047 1 0] CreatePlaylist
  (while (< (`KismetArrayLibrary.Array_Length` (`self.Playlist`)) (`self.ToRemember`))
    (`KismetArrayLibrary.Array_Add` (`self.Playlist`) (`KismetMathLibrary.RandomIntegerInRange` 0 3))))

(event `self.ReceiveTick`
  (params (DeltaSeconds :type "Float (single-precision)"))
  ;[1 1 1] DisplayWinCon
  (`self.SetWinLight`))

(event `SetWinLight`
  ;[1 1 1] DisplayWinCon
  (set `self.DisplayCounter` (`self.Difficulty`))
  (switch `int` (`self.DisplayCounter`)
    (:`1`
      (for _array_element (`self.IndicatorBP`)
        (`/Game/FPPuzzleGame/Blueprints/SimonSagtSachen/BP_IndicatorFlame.StopBurn` _array_element)))
    (:`2`
      (`/Game/FPPuzzleGame/Blueprints/SimonSagtSachen/BP_IndicatorFlame.Burn` (`|GetArrayItem` (`self.IndicatorBP`))))
    (:`3`
      (`/Game/FPPuzzleGame/Blueprints/SimonSagtSachen/BP_IndicatorFlame.Burn` (`|GetArrayItem` (`self.IndicatorBP`) 1)))
    (:`4`
      (`/Game/FPPuzzleGame/Blueprints/SimonSagtSachen/BP_IndicatorFlame.Burn` (`|GetArrayItem` (`self.IndicatorBP`) 2)))))

(event `Start`
  (bind _output (`|GetArrayItem` (`self.Playlist`) (`self.NotesPlayed`)))
  (if (`self.CanBePlayed`)
    (if (not (`self.isListening`))
      (set `self.isPlaying` true)
      (if (< (`self.NotesPlayed`) (`self.ToRemember`))
        (`KismetSystemLibrary.PrintString` "AmPlaying")
        (`/Game/FPPuzzleGame/Blueprints/SimonSagtSachen/BP_SimonFlameDispenser.StartFire` (`|GetArrayItem` (`self.FireDis`) _output) (+ _output 1))
        (set `self.NotesPlayed` (+ (`self.NotesPlayed`) 1))
        (if (< (`self.NotesPlayed`) (`self.ToRemember`))
          (`KismetSystemLibrary.Delay` (`self.Speed`))
          (`self.Start`)
          (else
            (set `self.isPlaying` false)
            (set `self.isListening` true)
            (`KismetSystemLibrary.Delay` 1.0)
            (message `/Game/FPPuzzleGame/Blueprints/Interfaces/BPI_Trigger.TriggerWithBool` (`self.BlendGenerate`) false)))))))

(event `AllowGenerateAgain`
  ;[1 0.7756 0.9124] Interaction
  (goto _label :!via `Reset`))

(event `ValueTrigger`
  (params (SwitchIntColor :type Integer))
  (bind _returnvalue (- (`self.SwitchIntColor`) 1))
  ;[1 0.7756 0.9124] Interaction
  (`|ExecutionSequence`
    (:`then_0`
      (bind _output_get (set `self.SwitchIntColor` SwitchIntColor)))
    (:`then_1`
      (switch `int` _output_get
        (:`0`
          (if (and (`self.isListening`) (`self.isPlaying`))
            (`KismetSystemLibrary.PrintString` "StillListeningandPlaying")
            (else
              (`/Engine/EditorBlueprintResources/StandardMacros.DoOnce` false :!label _label
                (:`Completed`
                  (message `/Game/FPPuzzleGame/Blueprints/Interfaces/BPI_Trigger.Trigger` (`self.BlendGenerate`))
                  (`self.SetupDifficulty`)
                  (`self.CreatePlaylist`)
                  (`KismetSystemLibrary.Delay` 2.0)
                  (`self.Start`))))))
        (:`1`
          (bind _isfail (`self.CheckNode` _returnvalue))
          ;;[0 0.5312 1] Blue
          (`self.PlayNotes` _isfail)
          (`self.CheckWin`))
        (:`2`
          (bind _isfail_2 (`self.CheckNode` _returnvalue))
          ;;[1 0.1068 0.1008] Red
          (`self.PlayNotes` _isfail_2)
          (`self.CheckWin`))
        (:`3`
          (bind _isfail_3 (`self.CheckNode` _returnvalue))
          ;;[0.4399 1 0.1922] Green
          (`self.PlayNotes` _isfail_3)
          (`self.CheckWin`))
        (:`4`
          (bind _isfail_4 (`self.CheckNode` _returnvalue))
          ;;[1 0.9191 0.05105] Yellow
          (`self.PlayNotes` _isfail_4)
          (`self.CheckWin`))))))

(event `/Game/FPPuzzleGame/Blueprints/Interfaces/BPI_Interact.Interact`
  ;[1 0.7756 0.9124] Interaction
)

(event `/Game/FPPuzzleGame/Blueprints/Interfaces/BPI_Interact.SetFocus`
  (params (IsFocused :type Boolean))
  ;[1 0.7756 0.9124] Interaction
)

(event `PlayNotes`
  (params (isFail :type Boolean))
  ;[1 0 0.6328] PlayNoteAnim
  (if isFail
    (for _array_element (`self.FireDis`)
      (`/Game/FPPuzzleGame/Blueprints/SimonSagtSachen/BP_SimonFlameDispenser.StartFire` _array_element 1))
    (`self.ResetMiniGame` true)))

(event `CheckWin`
  ;[1 0 0.4219] CheckWin
  (`self.SetWinLight`)
  (if (== (`KismetArrayLibrary.Array_Length` (`self.Playlist`)) (`KismetArrayLibrary.Array_Length` (`self.PlayerPlayList`)))
    (if (< (`self.Difficulty`) (`self.WinCondition(1-3)`))
      (message `/Game/FPPuzzleGame/Blueprints/Interfaces/BPI_Trigger.Trigger` (`self.BlendWinConPlusOne`))
      (`KismetSystemLibrary.Delay` 1.5)
      (`/Engine/EditorBlueprintResources/StandardMacros.IncrementInt` (`self.Difficulty`)
        (:`  `
          (`self.ResetMiniGame` false)))
      (else
        (`/Engine/EditorBlueprintResources/StandardMacros.IncrementInt` (`self.Difficulty`)
          (:`  `
            (for _array_element (`self.Actor`)
              (`/Engine/EditorBlueprintResources/StandardMacros.IsValid` _array_element
                (:`Is Valid`
                  (message `/Game/FPPuzzleGame/Blueprints/Interfaces/BPI_Puzzle.PuzzleSolved` _array_element)
                  (message `/Game/FPPuzzleGame/Blueprints/Interfaces/BPI_Trigger.Trigger` (`self.BlendWin`)))))))))))

(fn `CheckNode`
  (params (NoteToCheck :type Integer))
  (returns (isFail :type Boolean))
  (`KismetArrayLibrary.Array_Add` (`self.PlayerPlayList`) NoteToCheck)
  (return (not (== (`local.NoteToCheck`) (`|GetArrayItem` (`self.Playlist`) (- (`KismetArrayLibrary.Array_Length` (`self.PlayerPlayList`)) 1))))))

(fn `GetDisplayText`
  (returns (DisplayText :type String))
  (return ""))

(fn `ResetMiniGame`
  (params (isFail :type Boolean))
  (if isFail
    (set `self.isListening` false)
    (set `self.isPlaying` false)
    (`KismetArrayLibrary.Array_Clear` (`self.Playlist`))
    (set `self.NotesPlayed` 0)
    (set `self.ToRemember` 0)
    (bind _output_get (set `self.Difficulty` 1))
    (set `self.DisplayCounter` _output_get)
    (`KismetArrayLibrary.Array_Clear` (`self.PlayerPlayList`))
    (else
      (set `self.isListening` false)
      (set `self.isPlaying` false)
      (`KismetArrayLibrary.Array_Clear` (`self.Playlist`))
      (set `self.NotesPlayed` 0)
      (set `self.ToRemember` 0)
      (`KismetArrayLibrary.Array_Clear` (`self.PlayerPlayList`))))
  (`self.AllowGenerateAgain`))

(fn `UserConstructionScript`)