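; BP_LanternInteractable is an interactable lantern that offers a "to pickup" prompt, toggles physics simulation and can flare its orb's glow.
; Focus changes toggle custom depth on the mesh and call TriggerMessage on each valid referenced actor.
; LightItUp drives GlowIntensity on a construction-time dynamic material through a timeline, with a DoOnce gate that resets one second after it finishes.
; Interact is empty, and LightItUp prints a debug string.
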(event `self.ReceiveBeginPlay`
  (`TimelineComponent.SetPlayRate` (`self.ANIMLight`) 0.75))

(event `ActivatePhysics`
  (bind _output_get (set `self.IsSimulating` true))
  (`/Game/FPPuzzleGame/Blueprints/Interfaces/BPI_Grabable.SetSimulatePhysics` _output_get))

(event `DeactivatePhysics`
  (bind _output_get (set `self.IsSimulating` false))
  (`/Game/FPPuzzleGame/Blueprints/Interfaces/BPI_Grabable.SetSimulatePhysics` _output_get))

(event `self.SetFocus`
  (params (IsFocused :type Boolean))
  (`PrimitiveComponent.SetRenderCustomDepth` (`self.ItemPlacement`) IsFocused)
  (for _array_element (`self.ActorRef`)
    (`/Engine/EditorBlueprintResources/StandardMacros.IsValid` _array_element
      (:`Is Valid`
        (message `/Game/FPPuzzleGame/Blueprints/Interfaces/BPI_Trigger.Trigger` _array_element)))))

(event `self.Interact`)

(event `LightItUp`
  (`KismetSystemLibrary.PrintString` "BimBIMBAM")
  (`/Engine/EditorBlueprintResources/StandardMacros.DoOnce` false :!label _label
    (:`Completed`
      (bind (_direction _alpha) (`Timeline|ANIMLight` :!via `PlayFromStart`)
        (:`Update`
          (`MaterialInstanceDynamic.SetScalarParameterValue` (`self.MaterialInstance`) "GlowIntensity" (`KismetMathLibrary.Lerp` 3.0 100.0 _alpha)))
        (:`Finished`
          (`KismetSystemLibrary.Delay` 1.0)
          (`self.ResetTimeline`))))))

(event `self.ReceiveTick`
  (params (DeltaSeconds :type "Float (single-precision)")))

(event `ResetTimeline`
  (goto _label :!via `Reset`))

(fn `GetDisplayText`
  (returns (DisplayText :type String))
  (return "to pickup"))

(fn `UserConstructionScript`
  (bind _returnvalue (`PrimitiveComponent.CreateDynamicMaterialInstance` (`self.ItemPlacement`) 1 "/Game/FPPuzzleGame/Materials/OrbMaterials/M_OrbLantern.M_OrbLantern" "None"))
  (set `self.MaterialInstance` _returnvalue))