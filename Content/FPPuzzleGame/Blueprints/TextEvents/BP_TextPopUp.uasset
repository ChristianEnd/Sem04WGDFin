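; BP_TextPopUp shows a typewriter-style text pop-up on screen when its Trigger event fires.
; It creates a WBP_PopUpTypewriter widget with the full text and typing speed, optionally disabling player pawn input while it displays.
; A delay of text length times CharactersPerSecond (effectively used as seconds per character) plus a fixed buffer precedes restoring input and removing the widget.
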(event `/Game/FPPuzzleGame/Blueprints/Interfaces/BPI_Trigger.Trigger`
  (`self.PopUpText`))

(event `PopUpText`
  (bind _returnvalue (`GameplayStatics.GetPlayerController` 0))
  (bind _returnvalue_2 (`GameplayStatics.GetPlayerPawn` 0))
  (`|ExecutionSequence`
    (:`then_0`
      (set `self.HowLongToPauseInput` (+ (* (`KismetStringLibrary.Len` (`self.Full Text`)) (`self.Characters Per Second`)) 2.0)))
    (:`then_1`
      (bind _returnvalue_3 (`|CreateWidget` "/Game/FPPuzzleGame/UI/Widgets/WBP_PopUpTypewriter.WBP_PopUpTypewriter_C" (`GameplayStatics.GetPlayerController` 0) (`self.Characters Per Second`) (`self.Full Text`)))
      (bind _output_get (set `self.CreatedWidget` _returnvalue_3))
      (if (`self.ShouldBlockInput`)
        (`self.DisableInput` _returnvalue_2 _returnvalue))
      (`UserWidget.AddToViewport` _output_get 0)
      (`KismetSystemLibrary.Delay` (`self.HowLongToPauseInput`))
      (if (`self.ShouldBlockInput`)
        (`self.EnableInput` _returnvalue_2 _returnvalue))
      (`Widget.RemoveFromParent` _returnvalue_3))))

(fn `UserConstructionScript`)