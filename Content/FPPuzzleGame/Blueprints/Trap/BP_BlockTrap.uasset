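; Puzzle trap block that slides its Cube between its starting location and the Endposition location, both captured at BeginPlay.
; Activate alternates between two lerp timelines (Ani2, Timeline) through a FlipFlop, locked by a DoOnce until the move finishes.
; TriggerWithBool forwards to TWB: true plays Ani2, false plays Timeline through a start-closed DoOnce that reopens when Ani2 finishes.
; The Trigger function is an empty stub.
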(event `self.ReceiveBeginPlay`
  (set `self.StartLocation` (`SceneComponent.K2_GetComponentLocation` (`self.Cube`)))
  (set `self.MoveTo` (`SceneComponent.K2_GetComponentLocation` (`self.Endposition`))))

(event `/Game/FPPuzzleGame/Blueprints/Interfaces/BPI_Traps.Activate`
  (`/Engine/EditorBlueprintResources/StandardMacros.DoOnce` false :!label _label
    (:`Completed`
      (`/Engine/EditorBlueprintResources/StandardMacros.FlipFlop`
        (:`A`
          (bind (_direction _alpha) (`Timeline|Ani2` :!via `PlayFromStart` :!label _label_2)
            (:`Update`
              (`SceneComponent.K2_SetWorldLocation` (`self.Cube`) (`KismetMathLibrary.VLerp` (`self.StartLocation`) (`self.MoveTo`) _alpha) false false))
            (:`Finished`
              (`self.ResetTimeline`)
              (`self.BackAnimationActivate`))))
        (:`B`
          (bind (_direction_2 _alpha_2) (`Timeline|Timeline` :!via `PlayFromStart` :!label _label_3)
            (:`Update`
              (`SceneComponent.K2_SetWorldLocation` (`self.Cube`) (`KismetMathLibrary.VLerp` (`self.StartLocation`) (`self.MoveTo`) _alpha_2) false false))
            (:`Finished`
              (`self.ResetTimeline`))))))))

(event `ResetTimeline`
  (goto _label :!via `Reset`))

(event `TWB`
  (params (Condition :type Boolean))
  (if Condition
    (goto _label_2 :!via `PlayFromStart`)
    (else
      (`/Engine/EditorBlueprintResources/StandardMacros.DoOnce` true :!label _label_4
        (:`Completed`
          (goto _label_3 :!via `PlayFromStart`))))))

(event `BackAnimationActivate`
  (goto _label_4 :!via `Reset`))

(fn `Trigger`
  (return))

(fn `TriggerWithBool`
  (params (OnOff :type Boolean))
  (`self.TWB` OnOff)
  (return))

(fn `UserConstructionScript`)