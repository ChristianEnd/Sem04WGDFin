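; BP_CollisionTrigger is a one-shot trigger volume that fires linked actors when the player enters its box.
; On overlap it identifies the player through the BPI_Player interface, and a DoOnce limits it to a single activation.
; It then sends TriggerMessage to every actor in ActorToTrigger and optionally plays a level sequence.
; A separate Trigger event destroys the volume through DestroySelf.
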(event `self.Box.OnComponentBeginOverlap`
  (params (OverlappedComponent :type "PrimitiveComponent Object Reference") (OtherActor :type "Actor Object Reference") (OtherComp :type "PrimitiveComponent Object Reference") (OtherBodyIndex :type Integer) (bFromSweep :type Boolean) (SweepResult :type "HitResult Structure (by ref)"))
  (`/Engine/EditorBlueprintResources/StandardMacros.IsValid` OtherActor
    (:`Is Valid`
      (if (`KismetSystemLibrary.DoesImplementInterface` OtherActor "/Game/FPPuzzleGame/Blueprints/Interfaces/BPI_Player.BPI_Player_C")
        (`/Engine/EditorBlueprintResources/StandardMacros.DoOnce` false
          (:`Completed`
            (for _array_element (`self.ActorToTrigger`)
              (message `/Game/FPPuzzleGame/Blueprints/Interfaces/BPI_Trigger.Trigger` _array_element))
            (if (`self.ShouldPlaySequence`)
              (`MovieSceneSequencePlayer.Play` (`LevelSequenceActor.SequencePlayer` (`self.Sequence`))))))))))

(event `DestroySelf`
  (`self.K2_DestroyActor`))

(event `/Game/FPPuzzleGame/Blueprints/Interfaces/BPI_Trigger.Trigger`
  (`self.DestroySelf`))

(fn `UserConstructionScript`)