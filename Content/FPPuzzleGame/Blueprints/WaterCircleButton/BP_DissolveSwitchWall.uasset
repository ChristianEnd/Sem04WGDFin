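; A switchable puzzle wall that toggles between solid and hidden each time Trigger fires.
; IsDisabledOnStart sets whether it begins hidden, and FlipFlops alternate the state from there.
; Hiding turns off mesh collision and main-pass rendering instead of changing actor visibility, with no gradual dissolve in this graph.
; TriggerwithBool destroys the wall outright.
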(event `self.ReceiveBeginPlay`
  (bind _staticmeshcomponent (`self.StaticMeshComponent`))
  (if (`self.IsDisabledOnStart`)
    (`PrimitiveComponent.SetCollisionEnabled` _staticmeshcomponent "NoCollision" :!label _label)
    (`PrimitiveComponent.SetRenderInMainPass` _staticmeshcomponent false)))

(event `/Game/FPPuzzleGame/Blueprints/Interfaces/BPI_Trigger.Trigger`
  (bind _staticmeshcomponent (`self.StaticMeshComponent`))
  (bind _staticmeshcomponent_2 (`self.StaticMeshComponent`))
  (if (`self.IsDisabledOnStart`)
    (`/Engine/EditorBlueprintResources/StandardMacros.FlipFlop`
      (:`A`
        (`PrimitiveComponent.SetCollisionEnabled` _staticmeshcomponent "QueryAndPhysics")
        (`PrimitiveComponent.SetRenderInMainPass` _staticmeshcomponent true))
      (:`B`
        (goto _label)))
    (else
      (`/Engine/EditorBlueprintResources/StandardMacros.FlipFlop`
        (:`A`
          (`PrimitiveComponent.SetCollisionEnabled` _staticmeshcomponent_2 "NoCollision")
          (`PrimitiveComponent.SetRenderInMainPass` _staticmeshcomponent_2 false))
        (:`B`
          (`PrimitiveComponent.SetCollisionEnabled` _staticmeshcomponent_2 "QueryAndPhysics")
          (`PrimitiveComponent.SetRenderInMainPass` _staticmeshcomponent_2 true))))))

(event `/Game/FPPuzzleGame/Blueprints/Interfaces/BPI_Trigger.TriggerWithBool`
  (params (OnOff :type Boolean))
  (`self.K2_DestroyActor`))

(fn `UserConstructionScript`)