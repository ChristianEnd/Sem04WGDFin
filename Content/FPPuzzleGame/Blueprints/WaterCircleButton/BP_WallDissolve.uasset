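; BP_WallDissolve is a wall actor that dissolves away and destroys itself when its Trigger event is called.
; The construction script creates a dynamic instance of M_Dissolve_Red, which Trigger assigns to the mesh only when the dissolve starts.
; A timeline, slowed at BeginPlay, drives the material's Dissolve scalar from 1 to -1, then destroys the actor on finish.
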(event `self.ReceiveBeginPlay`
  (`TimelineComponent.SetPlayRate` (`self.Dissolve`) 0.25))

(event `/Game/FPPuzzleGame/Blueprints/Interfaces/BPI_Trigger.Trigger`
  (`PrimitiveComponent.SetMaterial` (`self.StaticMeshComponent`) 0 (`self.MaterialInstance`))
  (bind (_direction _alpha) (`Timeline|Dissolve` :!via `PlayFromStart`)
    (:`Update`
      (`MaterialInstanceDynamic.SetScalarParameterValue` (`self.MaterialInstance`) "Dissolve" (`KismetMathLibrary.Lerp` 1.0 -1.0 _alpha)))
    (:`Finished`
      (`self.K2_DestroyActor`))))

(fn `UserConstructionScript`
  (bind _returnvalue (`KismetMaterialLibrary.CreateDynamicMaterialInstance` "/Game/FPPuzzleGame/Materials/Translucent/M_Dissolve_Red.M_Dissolve_Red"))
  (set `self.MaterialInstance` _returnvalue))