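; BP_FunctionLibrary is a function library of inventory helpers for the puzzle game.
; OpenInventory pushes BP_InvRolando onto the gameplay stack through the first player controller's HUD and returns the cast result.
; AddItemToInventory and RemoveItemFromInventory find BP_Player by class lookup and forward the item and amount to its BPInventoryComponent.
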(fn `AddItemToInventory`
  (params (Item :type "DataTableRowHandle Structure") (Amount :type Integer))
  (bind _returnvalue (`GameplayStatics.GetActorOfClass` null "/Game/FPPuzzleGame/Blueprints/Player/BP_Player.BP_Player_C"))
  (`/Game/FPPuzzleGame/Blueprints/Components/BP_InventoryComponent.AddItem` (`/Game/FPPuzzleGame/Blueprints/Player/BP_Player.BP_InventoryComponent` _returnvalue) Item Amount))

(fn `OpenInventory`
  (returns (`AsBP Inv Rolando` :type "/Game/FPPuzzleGame/UI/Widgets/BP_InvRolando Object Reference"))
  (bind _pushedwidget (message `/Game/FPPuzzleGame/Blueprints/Interfaces/BPI_HUD.PushToGameplayStack` (`PlayerController.GetHUD` (`GameplayStatics.GetPlayerController` null)) "/Game/FPPuzzleGame/UI/Widgets/BP_InvRolando.BP_InvRolando_C"))
  (bind _asbp_inv_rolando (cast `/Game/FPPuzzleGame/UI/Widgets/BP_InvRolando` _pushedwidget))
  (return _asbp_inv_rolando))

(fn `RemoveItemFromInventory`
  (params (Item :type "DataTableRowHandle Structure (by ref)") (Amount :type Integer))
  (bind _returnvalue (`GameplayStatics.GetActorOfClass` null "/Game/FPPuzzleGame/Blueprints/Player/BP_Player.BP_Player_C"))
  (`/Game/FPPuzzleGame/Blueprints/Components/BP_InventoryComponent.RemoveItem` (`/Game/FPPuzzleGame/Blueprints/Player/BP_Player.BP_InventoryComponent` _returnvalue) Item Amount))