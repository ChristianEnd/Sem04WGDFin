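; Intro car actor with a door that swings open on trigger and starts an assigned level sequence.
; Trigger calls RotateDoor, which plays the sequence if valid and runs a slowed timeline rotating the door pivot.
; CloseDoor reverses that timeline; opening, closing and sequence playback are each guarded to happen only once.
; SetPhysics enables query and physics collision on the car's parts, and the display text is empty.
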(event `self.ReceiveBeginPlay`
  (`TimelineComponent.SetPlayRate` (`self.ANIMDoor`) 0.35))

(event `/Game/FPPuzzleGame/Blueprints/Interfaces/BPI_Trigger.Trigger`
  (`self.RotateDoor`))

(event `RotateDoor`
  (`self.PlaySequence`)
  (`/Engine/EditorBlueprintResources/StandardMacros.DoOnce` false
    (:`Completed`
      (bind (_direction _alpha) (`Timeline|ANIMDoor` :!via `PlayFromStart` :!label _label)
        (:`Update`
          (`SceneComponent.K2_SetRelativeRotation` (`self.Pivot`) (`KismetMathLibrary.RLerp` (struct) (struct :`Yaw` 70.0) _alpha true) false false))))))

(event `CloseDoor`
  (`/Engine/EditorBlueprintResources/StandardMacros.DoOnce` false
    (:`Completed`
      (goto _label :!via `ReverseFromEnd`))))

(event `PlaySequence`
  (bind _sequence (`self.Sequence`))
  (`/Engine/EditorBlueprintResources/StandardMacros.DoOnce` false
    (:`Completed`
      (`/Engine/EditorBlueprintResources/StandardMacros.IsValid` _sequence
        (:`Is Valid`
          (`MovieSceneSequencePlayer.Play` (`LevelSequenceActor.SequencePlayer` _sequence)))))))

(event `SetPhysics`
  (`PrimitiveComponent.SetCollisionEnabled` (`self.Car_RightDoor`) "QueryAndPhysics")
  (`PrimitiveComponent.SetCollisionEnabled` (`self.Car_Cube`) "QueryAndPhysics")
  (`PrimitiveComponent.SetCollisionEnabled` (`self.Car_CarFront`) "QueryAndPhysics")
  (`PrimitiveComponent.SetCollisionEnabled` (`self.Car_Tires_001`) "QueryAndPhysics")
  (`PrimitiveComponent.SetCollisionEnabled` (`self.Car_FrontInterior`) "QueryAndPhysics")
  (`PrimitiveComponent.SetCollisionEnabled` (`self.Pivot`) "QueryAndPhysics")
  (`PrimitiveComponent.SetCollisionEnabled` (`self.DoorHandleInteractable`) "QueryAndPhysics")
  (`PrimitiveComponent.SetCollisionEnabled` (`self.Cardoor`) "QueryAndPhysics")
  (`PrimitiveComponent.SetCollisionEnabled` (`self.Car_Tires`) "QueryAndPhysics"))

(fn `GetDisplayText`
  (returns (DisplayText :type String))
  (return ""))

(fn `UserConstructionScript`)