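; BP_RotatingRoom is a puzzle room whose circular walls rotate in two one-shot stages when triggered.
; BeginPlay stores the starting rotation, slows both timelines to quarter speed and disables interaction.
; Each TriggerwithBool call increments a counter: the first step rolls the walls from the stored rotation, the second eases them from their current world rotation toward zero.
; DoOnce gates keep each stage from replaying, with debug prints left in.
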(event `self.ReceiveBeginPlay`
  (`self.SetStartRotation`)
  (`self.CheckPlayRate`)
  (`self.SetInteractionDisabled`))

(event `SetStartRotation`
  (set `self.StartRot` (`SceneComponent.K2_GetComponentRotation` (`self.CircularRoomTest_Walls`))))

(event `CheckPlayRate`
  (`TimelineComponent.SetPlayRate` (`self.Ani01`) 0.25)
  (`TimelineComponent.SetPlayRate` (`self.Ani02`) 0.25))

(event `/Game/FPPuzzleGame/Blueprints/Interfaces/BPI_Trigger.TriggerWithBool`
  (params (OnOff :type Boolean))
  (`KismetSystemLibrary.PrintString` "1")
  (bind _result (`/Engine/EditorBlueprintResources/StandardMacros.IncrementInt` (`self.PositionToInt`))
    (:`  `
      (switch `int` _result
        (:`1`
          (`/Engine/EditorBlueprintResources/StandardMacros.DoOnce` false
            (:`Completed`
              (`KismetSystemLibrary.PrintString` "2")
              (bind (_direction _alpha) (`Timeline|Ani01` :!via `PlayFromStart`)
                (:`Update`
                  (`SceneComponent.K2_SetRelativeRotation` (`self.CircularRoomTest_Walls`) (`KismetMathLibrary.RLerp` (`self.StartRot`) (struct :`Yaw` 270.0) _alpha) false false))))))
        (:`2`
          (`/Engine/EditorBlueprintResources/StandardMacros.DoOnce` false
            (:`Completed`
              (`KismetSystemLibrary.PrintString` "3")
              (bind (_direction_2 _alpha_2) (`Timeline|Ani02` :!via `PlayFromStart`)
                (:`Update`
                  (`SceneComponent.K2_SetWorldRotation` (`self.CircularRoomTest_Walls`) (`KismetMathLibrary.RLerp` (`SceneComponent.K2_GetComponentRotation` (`self.CircularRoomTest_Walls`)) (struct) _alpha_2) false false))))))))))

(fn `UserConstructionScript`
  (`parent.UserConstructionScript`))